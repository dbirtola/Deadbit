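; Behavior tree service for Bits that picks a random location around their owner and stores it in the blackboard.
; On each AI tick it reads the owner actor from the blackboard and offsets that actor's location by a random normalized direction scaled by Range.
; The direction is confined to the XY plane, so the target stays at the owner's height and the Bit does not fly too high or low.
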(event EventReceiveTickAI
  (params (OwnerController :type AI%20Controller%20Object%20Reference) (ControlledPawn :type Pawn%20Object%20Reference) (DeltaSeconds :type Float%20%28single-precision%29))
  (bind _asactor (Utilities|Casting|CastToActor (Class|BTFunctionLibrary|GetBlackboardValueasObject (Variables|Default|GetOwnerKey))))
  (AI|BehaviorTree|SetBlackboardValueasVector (Variables|Default|GetRandomVectorKey) (+ (Transformation|GetActorLocation _asactor) (* (Math|Vector|Normalize (Math|Vector|MakeVector (Math|Random|RandomFloatinRange -1.0 1.0) (Math|Random|RandomFloatinRange -1.0 1.0) 0.0)) (Variables|Default|GetRange)))))