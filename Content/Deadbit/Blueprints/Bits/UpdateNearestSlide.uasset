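; Behavior tree service that finds the BitsSlide actor nearest to the AI-controlled pawn.
; On activation it loops over every BitsSlide in the level, comparing straight-line distance against a stored nearest distance.
; It writes the closest one found to a blackboard object key.
; The graph never resets the stored distance or actor before the search.
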(event EventReceiveActivationAI
  (params (OwnerController :type AI%20Controller%20Object%20Reference) (ControlledPawn :type Pawn%20Object%20Reference))
  (bind _outactors (Actor|GetAllActorsOfClass "/Game/Deadbit/Blueprints/Scenic/BitsSlide.BitsSlide_C"))
  (for _array_element _outactors
    (if (< (Math|Vector|VectorLength (- (Transformation|GetActorLocation _array_element) (Transformation|GetActorLocation ControlledPawn))) (Variables|Default|GetNearestDistance))
      (Variables|Default|SetNearestDistance (Math|Vector|VectorLength (- (Transformation|GetActorLocation _array_element) (Transformation|GetActorLocation ControlledPawn))))
      (Variables|Default|SetNearestSoFar _array_element)))
  (Class|BTFunctionLibrary|SetBlackboardValueasObject (Variables|Default|GetObjectKey) (Variables|Default|GetNearestSoFar)))