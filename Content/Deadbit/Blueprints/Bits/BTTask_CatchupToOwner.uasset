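; Behavior Tree task that snaps a Bit AI actor back to its owner, both read from blackboard keys.
; Each tick it succeeds if the two are within FinalDistance, otherwise it teleports the self actor to the owner's location without sweeping.
; Gradual CatchupSpeed-based movement nodes remain in the graph but are disconnected, and the execute event is empty.
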(event EventReceiveExecuteAI
  (params (OwnerController :type AI%20Controller%20Object%20Reference) (ControlledPawn :type Pawn%20Object%20Reference)))

(event EventTick
  (params (OwnerActor :type Actor%20Object%20Reference) (DeltaSeconds :type Float%20%28single-precision%29))
  (bind _ownerkey (Variables|Default|GetOwnerKey))
  (bind _selfkey (Variables|Default|GetSelfKey))
  (bind _returnvalue (AI|BehaviorTree|GetBlackboardValueasActor _selfkey))
  (bind _returnvalue_2 (AI|BehaviorTree|GetBlackboardValueasActor _ownerkey))
  (bind _returnvalue_3 (Transformation|GetActorLocation _returnvalue_2))
  (if (<= (Math|Vector|VectorLength (- _returnvalue_3 (Transformation|GetActorLocation _returnvalue))) (Variables|Default|GetFinalDistance))
    (AI|BehaviorTree|FinishExecute true)
    (else
      (Transformation|SetActorLocation _returnvalue _returnvalue_3 false true))))