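; Bits is a flying character whose mesh hovers and bobs, with a hum while it moves.
; BeginPlay sets Flying movement, and each Tick eases the mesh toward a sine/cosine offset with random jitter, or back to its origin when ShouldHover is off.
; While hovering, Humm follows velocity.
; An emote sound event exists, but its random-interval looping timer is disconnected.
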(event Custom|Make%20Emote%20Sound
  (Audio|PlaySoundatLocation "/Game/Deadbit/Sound/SoundCues/Bits/BitsEmote.BitsEmote" (Transformation|GetActorLocation) "0, 0, 0" 1.0 1.0 0.0 0 0 0))

(event EventTick
  (params (DeltaSeconds :type Float%20%28single-precision%29))
  (bind _staticmesh (Variables|Default|GetStaticMesh))
  (bind _humm (Variables|Default|GetHumm))
  (if (Variables|Default|GetShouldHover)
    (Transformation|SetRelativeLocation _staticmesh (Math|Vector|Lerp(Vector) (Variables|/Script/Engine.SceneComponent|GetRelativeLocation _staticmesh) (Math|Vector|MakeVector 0.0 (* (- (Math|Trig|Cos(Radians) (* (Utilities|Time|GetTimeSeconds) (Variables|Default|GetHoverFrequency))) (/ (Math|Trig|Cos(Radians) (* (Math|Random|RandomFloat) (Variables|Default|GetHoverVariation))) 2.0)) (Variables|Default|GetHoverAmplitude)) (+ (Variables|Default|GetHoverHeight) (* (Math|Trig|Sin(Radians) (* (Utilities|Time|GetTimeSeconds) (Variables|Default|GetHoverFrequency))) (Variables|Default|GetHoverAmplitude)))) (* DeltaSeconds 6.0)) false false)
    (if (> (Math|Vector|VectorLength (Transformation|GetVelocity)) 0.0)
      (if (not (Audio|Components|Audio|IsPlaying _humm))
        (Audio|Components|Audio|Play _humm 0.0))
      (else
        (Audio|Components|Audio|Stop _humm)))
    (else
      (Transformation|SetRelativeLocation (Variables|Default|GetStaticMesh) (Math|Vector|Lerp(Vector) (Variables|/Script/Engine.SceneComponent|GetRelativeLocation (Variables|Default|GetStaticMesh)) "0, 0, 0" 0.1) false false))))

(event EventBeginPlay
  (Pawn|Components|CharacterMovement|SetMovementMode (Variables|Character|GetCharacterMovement) "MOVE_Flying" 0))

(fn ConstructionScript)