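; Function library that converts chip-based code programs between chip grids, program structs and serialized string arrays, plus an actor-to-RobotPart array cast helper.
; ProgramsTable maps code piece classes to row-name IDs, which are written with parameters and hex-grid location as comma-separated entries.
; Parsers rebuild chip structs or ChipWidgetOld grids from these strings.
; ProgramStructToString saves only two connector directions per chip; ProgramToStrings omits them, though parsers read that field.
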(fn CastActorArraytoPartsArray
  (params (Actors :type Array%20of%20Actor%20Object%20References))
  (for _array_element Actors
    (bind _asrobot_part (Utilities|Casting|CastToRobotPart _array_element))
    (Utilities|Array|Add (LocalVariables|GetParts) _asrobot_part))
  (return (LocalVariables|GetParts)))

(fn ProgramtoStrings
  (params (Program%20Name :type String) (Program%20Structure :type Map%20of%20Int%20Point%20Structures%20to%20Objects))
  (bind _piecestrings (LocalVariables|GetPieceStrings))
  (Utilities|FlowControl|Sequence
    (:then_0
      (Utilities|Array|Add _piecestrings "{")
      (Utilities|Array|Add _piecestrings Program%20Name))
    (:then_1
      (bind _keys (Utilities|Map|Keys Program%20Structure))
      (for _array_element _keys
        (LocalVariables|SetCurrentCodePiece (Variables|/Game/Deadbit/Blueprints/UI/ProgrammingUI/ChipWidgetOld.ChipWidgetOld_C|GetCodePiece (.Value (Utilities|Map|Find Program%20Structure _array_element))))
        (LocalVariables|SetParameter1ID "-1")
        (LocalVariables|SetParameter2ID "-1")
        (Utilities|FlowControl|Sequence
          (:then_0
            ;[1 1 1] Store the parameters UniqueID's here to make the code cleaner since they need validity checks
            (if (> (Utilities|Array|Length (Variables|/Game/Deadbit/Blueprints/BotProgramming/Functions/BaseClasses/CodePiece.CodePiece_C|GetParameters (LocalVariables|GetCurrentCodePiece))) 0)
              (bind _identifier (CallFunction|GetIdentifierbyCodePieceClass (Utilities|GetClass (Utilities|Array|Get(acopy) (Variables|/Game/Deadbit/Blueprints/BotProgramming/Functions/BaseClasses/CodePiece.CodePiece_C|GetParameters (LocalVariables|GetCurrentCodePiece))))))
              (LocalVariables|SetParameter1ID _identifier)
              (if (> (Utilities|Array|Length (Variables|/Game/Deadbit/Blueprints/BotProgramming/Functions/BaseClasses/CodePiece.CodePiece_C|GetParameters (LocalVariables|GetCurrentCodePiece))) 1)
                (bind _identifier_2 (CallFunction|GetIdentifierbyCodePieceClass (Utilities|GetClass (Utilities|Array|Get(acopy) (Variables|/Game/Deadbit/Blueprints/BotProgramming/Functions/BaseClasses/CodePiece.CodePiece_C|GetParameters (LocalVariables|GetCurrentCodePiece)) 1))))
                (LocalVariables|SetParameter2ID _identifier_2))))
          (:then_1
            (bind _identifier_3 (CallFunction|GetIdentifierbyCodePieceClass (Utilities|GetClass (LocalVariables|GetCurrentCodePiece))))
            (Utilities|Array|Add (LocalVariables|GetPieceStrings) (Utilities|String|Append _identifier_3 "," (LocalVariables|GetParameter1ID) "," (LocalVariables|GetParameter2ID) "," (Utilities|String|ToString(Integer) (.X (Utilities|Struct|BreakIntPoint _array_element))) "," (Utilities|String|ToString(Integer) (.Y (Utilities|Struct|BreakIntPoint _array_element)))))))))
    (:then_2
      (Utilities|Array|Add (LocalVariables|GetPieceStrings) "}")
      (return (LocalVariables|GetPieceStrings)))))

(fn StringstoProgram
  (params (Strings :type Array%20of%20Strings))
  (Utilities|FlowControl|Sequence
    (:then_0
      (Utilities|Array|RemoveItem Strings "{")
      (Utilities|Array|RemoveItem Strings "}")
      (LocalVariables|SetProgram%20Name (Utilities|Array|Get(acopy) Strings))
      (Utilities|Array|RemoveIndex Strings)
      (for _array_element Strings
        (bind _chip_struct (CallFunction|ConstructChipStructfromStrings (Utilities|Array|Get(acopy) (Utilities|String|ParseIntoArray _array_element "," false)) (Utilities|Array|Get(acopy) (Utilities|String|ParseIntoArray _array_element "," false) 1) (Utilities|Array|Get(acopy) (Utilities|String|ParseIntoArray _array_element "," false) 2) (Utilities|Array|Get(acopy) (Utilities|String|ParseIntoArray _array_element "," false) 3) (Utilities|Array|Get(acopy) (Utilities|String|ParseIntoArray _array_element "," false) 4) (Utilities|String|ParseIntoArray (Utilities|Array|Get(acopy) (Utilities|String|ParseIntoArray _array_element "," false) 5) "-")))
        (bind _returnvalue (UserInterface|CreateWidget "/Game/Deadbit/Blueprints/UI/ProgrammingUI/ChipWidgetOld.ChipWidgetOld_C" 0 0))
        (bind _output_get (Variables|/Game/Deadbit/Blueprints/UI/ProgrammingUI/ChipWidgetOld.ChipWidgetOld_C|SetLocation _returnvalue (.Location (Utilities|Struct|BreakChipStruct _chip_struct))))
        (Default|InitializewithChipStruct _returnvalue _chip_struct)
        (Utilities|Map|Add (LocalVariables|GetProgram%20Structure) _output_get _returnvalue)))
    (:then_1
      (return (LocalVariables|GetProgram%20Name) (LocalVariables|GetProgram%20Structure)))))

(fn GetCodePieceClassbyIdentifier
  (params (UniqueID :type String))
  (bind _returnvalue (Utilities|GetDataTableRow "/Game/Deadbit/Blueprints/BotProgramming/ProgramsTable.ProgramsTable" (Utilities|String|StringToName UniqueID))
    (:then
      (return (Utilities|Struct|BreakProgramTableRow _returnvalue)))))

(fn GetIdentifierbyCodePieceClass
  (params (Code%20Piece%20Class :type Code%20Piece%20Class%20Reference))
  (bind _outrownames (DataTable|GetDataTableRowNames "/Game/Deadbit/Blueprints/BotProgramming/ProgramsTable.ProgramsTable"))
  (for _array_element _outrownames
    (bind _returnvalue (Utilities|GetDataTableRow "/Game/Deadbit/Blueprints/BotProgramming/ProgramsTable.ProgramsTable" _array_element)
      (:then
        (if (== (Utilities|Struct|BreakProgramTableRow _returnvalue) Code%20Piece%20Class)
          (return (Utilities|String|ToString(Name) _array_element))))))
  (return "-1"))

(fn ConstructChipStructfromStrings
  (params (ChipID :type String) (Parameter1ID :type String) (Parameter2ID :type String) (X :type String) (Y :type String) (Connector%20Directions :type Array%20of%20Strings))
  (Utilities|FlowControl|Sequence
    (:then_0
      (if (Utilities|Enum|NotEqual(Enum) ChipID "-1")
        (bind _code_piece_class (CallFunction|GetCodePieceClassbyIdentifier ChipID))
        (LocalVariables|SetBase%20Chip _code_piece_class)))
    (:then_1
      (if (Utilities|Enum|NotEqual(Enum) Parameter1ID "-1")
        (bind _code_piece_class_2 (CallFunction|GetCodePieceClassbyIdentifier Parameter1ID))
        (LocalVariables|SetParameter%201 _code_piece_class_2)))
    (:then_2
      (if (Utilities|Enum|NotEqual(Enum) Parameter2ID "-1")
        (bind _code_piece_class_3 (CallFunction|GetCodePieceClassbyIdentifier Parameter2ID))
        (LocalVariables|SetParameter2 _code_piece_class_3)))
    (:then_3
      (for _array_element Connector%20Directions
        (Utilities|Array|Add (LocalVariables|GetDirections) (Utilities|Enum|ByteToEnumHexDirection (Math|Conversions|ToByte(Integer) (Math|Conversions|ToInteger(Byte) _array_element))))))
    (:then_4
      (return (Utilities|Struct|MakeChipStruct (LocalVariables|GetBase%20Chip) (LocalVariables|GetParameter%201) (LocalVariables|GetParameter2) (Utilities|Struct|MakeIntPoint (Math|Conversions|ToInteger(Byte) X) (Math|Conversions|ToInteger(Byte) Y)) (LocalVariables|GetDirections))))))

(fn ConstructProgramStructfromStrings
  (params (Strings :type Array%20of%20Strings))
  (Utilities|FlowControl|Sequence
    (:then_0
      (Utilities|Array|RemoveItem Strings "{")
      (Utilities|Array|RemoveItem Strings "}")
      (LocalVariables|SetProgram%20Name (Utilities|Array|Get(acopy) Strings))
      (Utilities|Array|RemoveIndex Strings)
      (for _array_element Strings
        (bind _chip_struct (CallFunction|ConstructChipStructfromStrings (Utilities|Array|Get(acopy) (Utilities|String|ParseIntoArray _array_element "," false)) (Utilities|Array|Get(acopy) (Utilities|String|ParseIntoArray _array_element "," false) 1) (Utilities|Array|Get(acopy) (Utilities|String|ParseIntoArray _array_element "," false) 2) (Utilities|Array|Get(acopy) (Utilities|String|ParseIntoArray _array_element "," false) 3) (Utilities|Array|Get(acopy) (Utilities|String|ParseIntoArray _array_element "," false) 4) (Utilities|String|ParseIntoArray (Utilities|Array|Get(acopy) (Utilities|String|ParseIntoArray _array_element "," false) 5) "-")))
        (Utilities|Array|Add (LocalVariables|GetChipStructs) _chip_struct)))
    (:then_1
      (return (Utilities|Struct|MakeProgramStruct (LocalVariables|GetProgram%20Name) (LocalVariables|GetChipStructs))))))

(fn GetProgramfromStruct
  (params (Program%20Struct :type Program%20Struct%20Structure))
  (bind (_programname _chips) (Utilities|Struct|BreakProgramStruct Program%20Struct))
  (for _array_element _chips
    (bind _returnvalue (UserInterface|CreateWidget "/Game/Deadbit/Blueprints/UI/ProgrammingUI/ChipWidgetOld.ChipWidgetOld_C" 0 0))
    (bind _output_get (Variables|/Game/Deadbit/Blueprints/UI/ProgrammingUI/ChipWidgetOld.ChipWidgetOld_C|SetLocation _returnvalue (.Location (Utilities|Struct|BreakChipStruct _array_element))))
    (Default|InitializewithChipStruct _returnvalue _array_element)
    (Utilities|Map|Add (LocalVariables|GetProgram%20Structure) _output_get _returnvalue))
  (return _programname (LocalVariables|GetProgram%20Structure)))

(fn ConstructProgramStructfromGrid
  (params (Name :type String) (ProgramGrid :type Map%20of%20Int%20Point%20Structures%20to%20Objects))
  (bind _keys (Utilities|Map|Keys ProgramGrid))
  (for _array_element _keys
    (LocalVariables|SetCurrent%20Code%20Piece (Variables|/Game/Deadbit/Blueprints/UI/ProgrammingUI/ChipWidgetOld.ChipWidgetOld_C|GetCodePiece (.Value (Utilities|Map|Find ProgramGrid _array_element))))
    (for (_array_element_2 _array_index) (Variables|/Game/Deadbit/Blueprints/BotProgramming/Functions/BaseClasses/CodePiece.CodePiece_C|GetParameters (LocalVariables|GetCurrent%20Code%20Piece))
      (Utilities|IsValid _array_element_2
        (:Is%20Valid
          (switch int _array_index
            (:0
              (LocalVariables|SetParameter1 (Utilities|GetClass _array_element_2)))
            (:1
              (LocalVariables|SetParameter2 (Utilities|GetClass _array_element_2)))))))
    (Utilities|Array|Add (LocalVariables|GetChips) (Utilities|Struct|MakeChipStruct (Utilities|GetClass (LocalVariables|GetCurrent%20Code%20Piece)) (LocalVariables|GetParameter1) (LocalVariables|GetParameter2) _array_element (Variables|/Game/Deadbit/Blueprints/UI/ProgrammingUI/ChipWidgetOld.ChipWidgetOld_C|GetConnectorsDirections (.Value (Utilities|Map|Find ProgramGrid _array_element))))))
  (return (Utilities|Struct|MakeProgramStruct Name (LocalVariables|GetChips))))

(fn ProgramStructtoString
  (params (Program%20Struct :type Program%20Struct%20Structure))
  (bind (_programname _chips) (Utilities|Struct|BreakProgramStruct Program%20Struct))
  (LocalVariables|SetName _programname)
  (LocalVariables|SetChips _chips)
  (Utilities|FlowControl|Sequence
    (:then_0
      (Utilities|Array|Add (LocalVariables|GetStrings) "{")
      (Utilities|Array|Add (LocalVariables|GetStrings) (LocalVariables|GetName)))
    (:then_1
      (for _array_element (LocalVariables|GetChips)
        (if (Utilities|IsValidClass (.BasePiece (Utilities|Struct|BreakChipStruct _array_element)))
          (bind _identifier (CallFunction|GetIdentifierbyCodePieceClass (.BasePiece (Utilities|Struct|BreakChipStruct _array_element))))
          (bind _identifier_2 (CallFunction|GetIdentifierbyCodePieceClass (.Parameter1 (Utilities|Struct|BreakChipStruct _array_element))))
          (bind _identifier_3 (CallFunction|GetIdentifierbyCodePieceClass (.Parameter2 (Utilities|Struct|BreakChipStruct _array_element))))
          (Utilities|Array|Add (LocalVariables|GetStrings) (Utilities|String|Append _identifier "," _identifier_2 "," _identifier_3 "," (Utilities|String|ToString(Integer) (.X (Utilities|Struct|BreakIntPoint (.Location (Utilities|Struct|BreakChipStruct _array_element))))) "," (Utilities|String|ToString(Integer) (.Y (Utilities|Struct|BreakIntPoint (.Location (Utilities|Struct|BreakChipStruct _array_element))))) "," (Utilities|String|ToString(Integer) (Math|Conversions|ToInteger(Byte) (Utilities|Array|Get(acopy) (.ConnectorDirections (Utilities|Struct|BreakChipStruct _array_element))))) "-" (Utilities|String|ToString(Integer) (Math|Conversions|ToInteger(Byte) (Utilities|Array|Get(acopy) (.ConnectorDirections (Utilities|Struct|BreakChipStruct _array_element)) 1))))))))
    (:then_2
      (Utilities|Array|Add (LocalVariables|GetStrings) "}")
      (return (LocalVariables|GetStrings)))))