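; Elevator Blueprint that repositions the ChipBase01 component when something overlaps its Sensor.
; The overlap sets the Movement timeline's play rate to 50 divided by the distance to EndPoint, scaling speed to travel length, then plays it.
; Each update lerps from EndPoint (A) to the component's current location (B), re-read every tick rather than cached, without sweep.
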(event OnComponentBeginOverlap(Sensor)
  (params (OverlappedComponent :type Primitive%20Component%20Object%20Reference) (OtherActor :type Actor%20Object%20Reference) (OtherComp :type Primitive%20Component%20Object%20Reference) (OtherBodyIndex :type Integer) (bFromSweep :type Boolean) (SweepResult :type Hit%20Result%20Structure%20%28by%20ref%29))
  (bind _chip_base_01 (Variables|Default|GetChip_Base_01))
  (bind _endpoint (Variables|Default|GetEndPoint))
  (bind _returnvalue (Transformation|GetWorldLocation _chip_base_01))
  (Components|Timeline|SetPlayRate (Variables|Default|GetMovement) (/ 5e+01 (Math|Vector|VectorLength (- _endpoint _returnvalue))))
  (bind _movement (Timeline|Movement Play)
    (:Update
      (Transformation|SetWorldLocation (Variables|Default|GetChip_Base_01) (Math|Vector|Lerp(Vector) _endpoint _returnvalue _movement) false false))))

(fn ConstructionScript)