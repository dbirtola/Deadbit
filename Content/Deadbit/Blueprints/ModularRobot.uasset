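; ModularRobot is a programmable robot that runs programs in response to gameplay events.
; On BeginPlay it takes the first ThirdPersonCharacter as owner, spawns an EventQueue with enemy-spotted and took-damage events, and binds one ProgramFactory template program to both.
; Damage and sphere overlaps by any ThirdPersonCharacter invoke those events.
; GetAvailableCodePieces returns a hardcoded instruction list; robot-part grants and older manual program assembly are disconnected.
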(event OnComponentBeginOverlap(Sphere)
  (params (OverlappedComponent :type Primitive%20Component%20Object%20Reference) (OtherActor :type Actor%20Object%20Reference) (OtherComp :type Primitive%20Component%20Object%20Reference) (OtherBodyIndex :type Integer) (bFromSweep :type Boolean) (SweepResult :type Hit%20Result%20Structure%20%28by%20ref%29))
  (Utilities|Casting|CastToThirdPersonCharacter OtherActor)
  (Default|Invoke (Variables|Default|GetEnemySpottedEvent)))

(event Custom|TakeDamageEvent
  (Default|Invoke (Variables|Default|GetTookDamageEvent)))

(event EventBeginPlay
  (bind _outactors (Actor|GetAllActorsOfClass "/Game/Deadbit/Blueprints/ThirdPersonCharacter.ThirdPersonCharacter_C"))
  (Actor|SetOwner (Utilities|Array|Get(acopy) _outactors))
  (bind _returnvalue (Game|SpawnActorfromClass "/Game/Deadbit/Blueprints/BotProgramming/EventQueue.EventQueue_C" (Math|Transform|MakeTransform "0, 0, 0" "0, 0, 0" "1,1,1") "Undefined" 0 0))
  (bind _output_get (Variables|Default|SetEventQueue _returnvalue))
  (bind _returnvalue_2 (Game|SpawnActorfromClass "/Game/Deadbit/Blueprints/BotProgramming/Events/EnemySpottedEvent.EnemySpottedEvent_C" (Math|Transform|MakeTransform "0, 0, 0" "0, 0, 0" "1,1,1") "Undefined" 0 0))
  (bind _output_get_2 (Variables|Default|SetEnemySpottedEvent _returnvalue_2))
  (bind _returnvalue_3 (Game|SpawnActorfromClass "/Game/Deadbit/Blueprints/BotProgramming/Events/TookDamageEvent.TookDamageEvent_C" (Math|Transform|MakeTransform "0, 0, 0" "0, 0, 0" "1,1,1") "Undefined" 0 0))
  (bind _output_get_3 (Variables|Default|SetTookDamageEvent _returnvalue_3))
  (Utilities|Array|Add (Variables|/Game/Deadbit/Blueprints/BotProgramming/EventQueue.EventQueue_C|GetEvents _output_get) _returnvalue_2)
  (Utilities|Array|Add (Variables|/Game/Deadbit/Blueprints/BotProgramming/EventQueue.EventQueue_C|GetEvents _output_get) _output_get_3)
  (bind _outactors_2 (Actor|GetAllActorsOfClass "/Game/Deadbit/Blueprints/BotProgramming/ProgramFactory.ProgramFactory_C"))
  (bind _program (Default|CreateProgramfromTemplate (Utilities|Array|Get(acopy) _outactors_2) "NewEnumerator2" self))
  (Utilities|Array|Add (Variables|Default|GetPrograms) _program)
  (Default|BindProgramtoEvent _output_get_2 _program)
  (Default|BindProgramtoEvent _output_get_3 _program)
  (Variables|/Game/Deadbit/Blueprints/BotProgramming/Program.Program_C|SetOwningCharacter _program (Components|GetOwner)))

(fn ConstructionScript)

(fn GetAvailableCodePieces
  (bind _output_get (LocalVariables|SetTemp (Utilities|Array|MakeArray "/Game/Deadbit/Blueprints/BotProgramming/Functions/DestroyObjectsInstruction.DestroyObjectsInstruction_C" "/Game/Deadbit/Blueprints/BotProgramming/Functions/GetNearestEnemy.GetNearestEnemy_C" "/Game/Deadbit/Blueprints/BotProgramming/Functions/DoXInstruction.DoXInstruction_C" "/Game/Deadbit/Blueprints/BotProgramming/Functions/ShrinkObject.ShrinkObject_C")))
  (return (LocalVariables|GetTemp)))