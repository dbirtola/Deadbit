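; Projectile that recursively splits into pairs of new bullets on a looping timer that starts after an initial delay.
; Each split decrements SplitsLeft and passes it to two spawns with mirrored offset and angle, until zero pauses the timer and optionally destroys the actor.
; The Bidirectional/alternating Direction branch is disconnected, so splits always go both ways.
; CreateBulletTransform's offset-and-yaw transform math is also left unconnected.
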(event Custom|CustomEvent_0
  (CallFunction|SplitBullets))

(event EventBeginPlay
  (|CallParentFunction)
  (Variables|Default|Set_SplitsLeft (Variables|Default|GetnumOfSplits))
  (Utilities|FlowControl|Delay (Variables|Default|GetdelayBeforeInitialSplit))
  (bind _returnvalue (Utilities|Time|SetTimerbyEvent (delegate Custom|CustomEvent_0) (Variables|Default|GetsplitIntervals) true))
  (Variables|Default|Set_SplitFunctionTimer _returnvalue))

(event Collision|EventActorBeginOverlap
  (params (OtherActor :type Actor%20Object%20Reference)))

(event EventTick
  (params (DeltaSeconds :type Float%20%28single-precision%29)))

(fn ConstructionScript
  (|CallParentFunction))

(fn SplitBullets
  (bind _split_angle (Variables|Default|GetSplit%20Angle))
  (if (!= (Variables|Default|Get_SplitsLeft) 0)
    (Math|Integer|DecrementInt (Variables|Default|Get_SplitsLeft)
      (:%20%20
        (Utilities|FlowControl|Sequence ; Do Both
          (:then_0
            (bind _returnvalue (Game|SpawnActorfromClass "Bullet-Of-Recursion_C" (Utilities|CreateBulletTransform (Variables|Default|GetSpawnedBulletXOffset) _split_angle) "Undefined" 0 0))
            (Variables|Bullet-Of-Recursion_C|SetnumOfSplits _returnvalue (Variables|Default|Get_SplitsLeft)))
          (:then_1
            (bind _returnvalue_2 (Game|SpawnActorfromClass "Bullet-Of-Recursion_C" (Utilities|CreateBulletTransform (* (Variables|Default|GetSpawnedBulletXOffset) -1) (* _split_angle -1.0)) "Undefined" 0 0))
            (Variables|Bullet-Of-Recursion_C|SetnumOfSplits _returnvalue_2 (Variables|Default|Get_SplitsLeft))))))
    (else
      ;[1 1 1] Stop Spawning
      (Utilities|Time|PauseTimerbyHandle (Variables|Default|Get_SplitFunctionTimer))
      (if (Variables|Default|GetdestroyThisAfterLastSplit)
        (Actor|DestroyActor)))))