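; Projectile Blueprint that, after an initial delay, splits off bullets of a configurable class.
; BeginPlay sets the split budget and starts a timer on Split Bullets, which spawns angled bullets through Create Bullet Transform.
; Each split fires both sides when Bidirectional, otherwise alternates sides by flipping Direction.
; When Split Bullets runs with no splits left, it pauses the timer and optionally destroys the actor.
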(event EventBeginPlay
  (|CallParentFunction)
  (Variables|Default|Set_SplitsLeft (Variables|Default|GetnumOfSplits))
  (Utilities|FlowControl|Delay (Variables|Default|GetdelayBeforeInitialSplit))
  (bind _returnvalue (Utilities|Time|SetTimerbyFunctionName 0 "Split Bullets" (Variables|Default|GetsplitIntervals)))
  (Variables|Default|Set_SplitFunctionTimer _returnvalue))

(event Collision|EventActorBeginOverlap
  (params (OtherActor :type Actor%20Object%20Reference)))

(event EventTick
  (params (DeltaSeconds :type Float%20%28single-precision%29)))

(fn ConstructionScript
  (|CallParentFunction))

(fn SplitBullets
  (bind _split_angle (Variables|Default|GetSplit%20Angle))
  (bind _spawnablebullet (Variables|Default|GetSpawnableBullet))
  (if (!= (Variables|Default|Get_SplitsLeft) 0)
    (Math|Integer|DecrementInt (Variables|Default|Get_SplitsLeft)
      (:%20%20
        (if (Variables|Default|GetBidirectional)
          (Utilities|FlowControl|Sequence ; Do Both
            (:then_0
              (Game|SpawnActorfromClass _spawnablebullet (Utilities|CreateBulletTransform _split_angle) "Undefined" 0 0 :!label _label))
            (:then_1
              (Game|SpawnActorfromClass _spawnablebullet (Utilities|CreateBulletTransform (* _split_angle -1.0)) "Undefined" 0 0 :!label _label_2)))
          (elif (Variables|Default|Get_direction)
            (Variables|Default|Set_direction (not (Variables|Default|Get_direction)))
            (goto _label)
            (else
              (Variables|Default|Set_direction (not (Variables|Default|Get_direction)))
              (goto _label_2))))))
    (else
      ;[1 1 1] Stop Spawning
      (Utilities|Time|PauseTimerbyHandle (Variables|Default|Get_SplitFunctionTimer))
      (if (Variables|Default|GetdestroyThisAfterLastSplit)
        (Actor|DestroyActor)))))