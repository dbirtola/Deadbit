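; HomingBullet is a projectile that starts homing on a target, by default the player, after a configurable delay.
; On BeginPlay it waits, falls back to the first PlayerCharacter found if no valid HomingTarget exists, then enables homing on its ProjectileMovement.
; It adds a scene component slightly above the target's origin as the homing point.
; The bullet destroys itself shortly after homing begins.
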(event EventBeginPlay
  (bind _projectilemovement (Variables|Default|GetProjectileMovement))
  (|CallParentFunction)
  (Utilities|FlowControl|Delay (Variables|Default|GetDelayBeforeHoming))
  (Utilities|IsValid (Variables|Default|GetHomingTarget)
    (:Is%20Valid
      _)
    (:Is%20Not%20Valid
      (Utilities|FindPlayerandSetasHomingTarget)))
  (Variables|/Script/Engine.ProjectileMovementComponent|SetbIsHomingProjectile _projectilemovement true)
  (bind _scene_component (Utilities|CreateSceneComponentAbovePlayer))
  (Variables|/Script/Engine.ProjectileMovementComponent|SetHomingTargetComponent _projectilemovement _scene_component)
  (Variables|/Script/Engine.ProjectileMovementComponent|SetHomingAccelerationMagnitude _projectilemovement 2e+03)
  (Utilities|FlowControl|Delay 1.5)
  (Actor|DestroyActor))

(event Collision|EventActorBeginOverlap
  (params (OtherActor :type Actor%20Object%20Reference)))

(event EventTick
  (params (DeltaSeconds :type Float%20%28single-precision%29)))

(fn ConstructionScript
  (|CallParentFunction))