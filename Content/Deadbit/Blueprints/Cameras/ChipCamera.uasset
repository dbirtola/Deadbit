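; ChipCamera is a camera Blueprint that finds which Chip lies under a given screen position.
; GetActorClicked builds a ray end point by hand, using fixed-angle tangents and the ortho far clip distance to map screen fractions onto world X/Y offsets.
; It traces WorldDynamic objects from the camera, returning the hit location and any Chip hit.
; The event graph holds only an unconnected deprojection trace with debug printing.
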(fn ConstructionScript)

(fn GetActorClicked
  (params (Screen%20X :type Float%20%28single-precision%29) (Screen%20Y :type Float%20%28single-precision%29))
  (bind _desiredview (Class|CameraComponent|GetCameraView (Variables|CameraActor|GetCameraComponent) 0.0))
  (bind _outhit (Collision|LineTraceForObjects (.location _desiredview) (* (Math|Vector|MakeVector (+ (.X (Math|Vector|BreakVector (Math|Vector|MakeVector (- (.X (Math|Vector|BreakVector (+ (.location _desiredview) (* (Math|Vector|GetForwardVector (.rotation _desiredview)) (.orthofarclipplane _desiredview))))) (* (Math|Trig|Tan(Degrees) -37.0) (.orthofarclipplane _desiredview))) (- (.Y (Math|Vector|BreakVector (+ (.location _desiredview) (* (Math|Vector|GetForwardVector (.rotation _desiredview)) (.orthofarclipplane _desiredview))))) (* (Math|Trig|Tan(Degrees) 45.0) (.orthofarclipplane _desiredview))) (.Z (Math|Vector|BreakVector (+ (.location _desiredview) (* (Math|Vector|GetForwardVector (.rotation _desiredview)) (.orthofarclipplane _desiredview)))))))) (* (* (* (Math|Trig|Tan(Degrees) -37.0) (.orthofarclipplane _desiredview)) 2.0) Screen%20Y)) (+ (.Y (Math|Vector|BreakVector (Math|Vector|MakeVector (- (.X (Math|Vector|BreakVector (+ (.location _desiredview) (* (Math|Vector|GetForwardVector (.rotation _desiredview)) (.orthofarclipplane _desiredview))))) (* (Math|Trig|Tan(Degrees) -37.0) (.orthofarclipplane _desiredview))) (- (.Y (Math|Vector|BreakVector (+ (.location _desiredview) (* (Math|Vector|GetForwardVector (.rotation _desiredview)) (.orthofarclipplane _desiredview))))) (* (Math|Trig|Tan(Degrees) 45.0) (.orthofarclipplane _desiredview))) (.Z (Math|Vector|BreakVector (+ (.location _desiredview) (* (Math|Vector|GetForwardVector (.rotation _desiredview)) (.orthofarclipplane _desiredview)))))))) (* (* (* (Math|Trig|Tan(Degrees) 45.0) (.orthofarclipplane _desiredview)) 2.0) Screen%20X)) (.Z (Math|Vector|BreakVector (Math|Vector|MakeVector (- (.X (Math|Vector|BreakVector (+ (.location _desiredview) (* (Math|Vector|GetForwardVector (.rotation _desiredview)) (.orthofarclipplane _desiredview))))) (* (Math|Trig|Tan(Degrees) -37.0) (.orthofarclipplane _desiredview))) (- (.Y (Math|Vector|BreakVector (+ (.location _desiredview) (* (Math|Vector|GetForwardVector (.rotation _desiredview)) (.orthofarclipplane _desiredview))))) (* (Math|Trig|Tan(Degrees) 45.0) (.orthofarclipplane _desiredview))) (.Z (Math|Vector|BreakVector (+ (.location _desiredview) (* (Math|Vector|GetForwardVector (.rotation _desiredview)) (.orthofarclipplane _desiredview))))))))) 1e+04) (Utilities|Array|MakeArray "ObjectTypeQuery2") false 0 "None"))
  (bind _aschip (Utilities|Casting|CastToChip (.HitActor (Collision|BreakHitResult _outhit)))
    (:then
      (return _aschip (.Location (Collision|BreakHitResult _outhit))))
    (:CastFailed
      (return 0 (.Location (Collision|BreakHitResult _outhit))))))