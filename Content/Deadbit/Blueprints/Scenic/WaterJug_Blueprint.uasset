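; Scenic water jug that starts leaking when its physics mesh wakes or is hit.
; Either event activates its particle system and starts a fast looping timer, with nothing here to stop it.
; Each tick traces straight down against WorldStatic objects and spawns a scaled-down puddle decal Blueprint with random yaw at the hit point.
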(event OnComponentWake(StaticMeshComponent)
  (params (WakingComponent :type Primitive%20Component%20Object%20Reference) (BoneName :type Name :default "None"))
  (Components|Activation|Activate (Variables|Default|GetParticleSystem) true)
  (Utilities|Time|SetTimerbyEvent (delegate Custom|Make%20Puddle) 0.4 true))

(event OnComponentHit(StaticMeshComponent)
  (params (HitComponent :type Primitive%20Component%20Object%20Reference) (OtherActor :type Actor%20Object%20Reference) (OtherComp :type Primitive%20Component%20Object%20Reference) (NormalImpulse :type Vector :default "0, 0, 0") (Hit :type Hit%20Result%20Structure%20%28by%20ref%29))
  (Components|Activation|Activate (Variables|Default|GetParticleSystem) true)
  (Utilities|Time|SetTimerbyEvent (delegate Custom|Make%20Puddle) 0.4 true))

(event Custom|Make%20Puddle
  (bind _returnvalue (Transformation|GetActorLocation))
  (bind (_x _y) (Math|Vector|BreakVector _returnvalue))
  (bind (_outhit _returnvalue_2) (Collision|LineTraceForObjects _returnvalue (Math|Vector|MakeVector _x _y -5e+03) (Utilities|Array|MakeArray "ObjectTypeQuery1") false 0 "None"))
  (if _returnvalue_2
    (Game|SpawnActorfromClass "/Game/Deadbit/Blueprints/Scenic/D_Lit_Puddle_Inst6_Blueprint.D_Lit_Puddle_Inst6_Blueprint_C" (Math|Transform|MakeTransform (.Location (Collision|BreakHitResult _outhit)) (Math|Rotator|MakeRotator 0.0 9e+01 (Math|Random|RandomFloatinRange 0.0 3.6e+02)) "0.600000,0.600000,0.600000") "Undefined" 0 0)))

(fn ConstructionScript)