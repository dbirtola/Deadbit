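; ChipPickup is a world pickup that grants the player a code piece when touched.
; A sphere overlap resolves the overlapping actor's instigator controller as a CBPlayerController and passes its configured DefaultClass to AddCodePieces with player notification.
; The actor then destroys itself and plays a 2D pickup sound.
; BeginPlay checks DefaultClass against a value but takes no action.
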(event OnComponentBeginOverlap(Sphere)
  (params (OverlappedComponent :type Primitive%20Component%20Object%20Reference) (OtherActor :type Actor%20Object%20Reference) (OtherComp :type Primitive%20Component%20Object%20Reference) (OtherBodyIndex :type Integer) (bFromSweep :type Boolean) (SweepResult :type Hit%20Result%20Structure%20%28by%20ref%29))
  (bind _ascbplayer_controller (Utilities|Casting|CastToCBPlayerController (Game|GetInstigatorController OtherActor)))
  (Default|AddCodePieces _ascbplayer_controller (Utilities|Array|MakeArray (Variables|Default|GetDefaultClass)) true)
  (Actor|DestroyActor)
  (Audio|PlaySound2D "/Game/Deadbit/Sound/SoundCues/PickupItem.PickupItem" 1.0 1.0 0.0 0 0))

(event EventBeginPlay
  (if (!= (Variables|Default|GetDefaultClass) 0)
    _))

(fn ConstructionScript)