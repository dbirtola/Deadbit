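; BitsSlide is a scenic slide actor that carries another actor along a spline.
; UseSlide accepts an actor only when none is sliding, resetting the distance to zero; its ApproachSpeed input is unused.
; Tick advances that distance by SlideSpeed, teleporting the rider to the spline's location and rotation.
; Past the spline's end, it releases the rider and calls SlideFinished.
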(event Custom|UseSlide
  (params (Actor :type Actor%20Object%20Reference) (Approach%20speed :type Float%20%28single-precision%29))
  (Utilities|IsValid (Variables|Default|GetActorSliding)
    (:Is%20Not%20Valid
      (bind _output_get (Variables|Default|SetActorSliding Actor))
      (Variables|Default|SetTargetPointAlongSlide 0.0))))

(event EventTick
  (params (DeltaSeconds :type Float%20%28single-precision%29))
  (Utilities|IsValid (Variables|Default|GetActorSliding)
    (:Is%20Valid
      (if (<= (Variables|Default|GetTargetPointAlongSlide) (Spline|GetSplineLength (Variables|Default|GetSpline)))
        (Variables|Default|SetTargetPointAlongSlide (+ (Variables|Default|GetTargetPointAlongSlide) (* (Variables|Default|GetSlide%20Speed) DeltaSeconds)))
        (Transformation|SetActorLocationAndRotation (Variables|Default|GetActorSliding) (Spline|GetLocationatDistanceAlongSpline (Variables|Default|GetSpline) (Variables|Default|GetTargetPointAlongSlide) "World") (Spline|GetRotationatDistanceAlongSpline (Variables|Default|GetSpline) (Variables|Default|GetTargetPointAlongSlide) "World") false true)
        (else
          (Variables|Default|SetActorSliding 0)
          (Variables|Default|SetTargetPointAlongSlide 0.0)
          (Default|CallSlideFinished))))))

(fn ConstructionScript)