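; A scenic vending machine that dispenses a random hat whenever it takes damage.
; Each hit spawns a random class from the hat list at the Scene component, makes it pickupable, enables mesh physics, launches it sideways and plays an impact effect.
; A class that fails the BasicHead cast only prints a joke warning.
; Once-only gating and explosion logic remain in the graph but are disconnected.
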(event Game|Damage|EventAnyDamage
  (params (Damage :type Float%20%28single-precision%29) (DamageType :type Damage%20Type%20Object%20Reference) (InstigatedBy :type Controller%20Object%20Reference) (DamageCauser :type Actor%20Object%20Reference))
  (bind _scene (Variables|Default|GetScene))
  (bind _returnvalue (Game|SpawnActorfromClass (Utilities|Array|Get(acopy) (Variables|Default|GetHatClass) (Math|Random|RandomIntegerinRange 0 (Utilities|-- (Utilities|Array|Length (Variables|Default|GetHatClass))))) (Math|Transform|MakeTransform (Transformation|GetWorldLocation (Variables|Default|GetScene)) "0, 0, 0" "1,1,1") "Undefined" 0 0))
  (bind _asbasic_head (Utilities|Casting|CastToBasicHead _returnvalue)
    (:then
      (Physics|SetSimulatePhysics (Variables|/Game/Deadbit/Blueprints/RobotParts/[Old]/BasicHead.BasicHead_C|GetHatMesh _asbasic_head) true)
      (Default|SetPickupable _returnvalue true)
      (Physics|SetPhysicsLinearVelocity (Variables|/Game/Deadbit/Blueprints/RobotParts/[Old]/BasicHead.BasicHead_C|GetHatMesh _asbasic_head) (* (Math|Vector|GetRightVector _scene) -4e+02) false "None")
      (Effects|SpawnEmitteratLocation "/Game/Deadbit/Cascade/P_GunArm_Impact.P_GunArm_Impact" (Transformation|GetWorldLocation _scene)))
    (:CastFailed
      (Development|PrintString "we only take hats in the vending machine sir"))))

(fn ConstructionScript)