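; StreetLamp23 is a scenic street lamp Blueprint that flickers its lamp material and a referenced spotlight.
; The construction script creates a dynamic instance of the street lamp material and applies it to the static mesh.
; Every tick, a sine-cosine product at two speeds drives the material's flicker parameter.
; The same wave, inverted, raised to a steep power and clamped to a narrow range, sets the spotlight intensity.
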(event EventTick
  (params (DeltaSeconds :type Float%20%28single-precision%29))
  (bind _returnvalue (Utilities|Time|GetTimeSeconds))
  (bind _returnvalue_2 (Utilities|Time|GetTimeSeconds))
  (bind _flicker_speed (Variables|Default|GetFlicker%20Speed))
  (bind _flickerspeed2 (Variables|Default|GetFlickerSpeed2))
  (bind _returnvalue_3 (* _returnvalue _flickerspeed2))
  (bind _returnvalue_4 (* _returnvalue_2 _flicker_speed))
  (bind _returnvalue_5 (Math|Trig|Sin(Radians) _returnvalue_4))
  (bind _returnvalue_6 (Math|Trig|Cos(Radians) _returnvalue_3))
  (bind _returnvalue_7 (* _returnvalue_5 _returnvalue_6))
  (Rendering|Material|SetScalarParameterValue (Variables|Default|GetDynamicMaterial) "BlueprintFlicker" _returnvalue_7 :!class /Script/Engine.MaterialInstanceDynamic)
  (Rendering|Components|Light|SetIntensity (Variables|/Script/Engine.SpotLight|GetSpotLightComponent (Variables|Default|GetLight)) (Math|Float|Clamp(Float) (Math|Float|Power (- 1.0 _returnvalue_7) 3e+01) 8.0 1e+01)))

(fn ConstructionScript
  (bind _returnvalue (Rendering|Material|CreateDynamicMaterialInstance "/Game/Deadbit/3D/Props/StreetLamp/M_StreetLamp_Inst.M_StreetLamp_Inst" "None" :!class /Script/Engine.KismetMaterialLibrary))
  (Variables|Default|SetDynamicMaterial _returnvalue)
  (Rendering|Material|SetMaterial (Variables|Debug|GetStaticMeshComponent) 0 _returnvalue))