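; Boss area trigger that lengthens the player's camera spring arm on the way toward the boss and restores it on the way back.
; Two boxes detect crossing direction: entering one arms a flag, and leaving the other consumes it.
; Crossing Box then Box2 plays the SpringArmExtension timeline, which drives TargetArmLength, while the opposite order reverses it.
; Any non-player actor entering a box clears that box's flag.
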(event OnComponentBeginOverlap(Box)
  (params (OverlappedComponent :type Primitive%20Component%20Object%20Reference) (OtherActor :type Actor%20Object%20Reference) (OtherComp :type Primitive%20Component%20Object%20Reference) (OtherBodyIndex :type Integer) (bFromSweep :type Boolean) (SweepResult :type Hit%20Result%20Structure%20%28by%20ref%29))
  (Utilities|Casting|CastToPlayerCharacter OtherActor
    (:then
      (Variables|Default|SetTowardsBoss true))
    (:CastFailed
      (Variables|Default|SetTowardsBoss false))))

(event OnComponentEndOverlap(Box2)
  (params (OverlappedComponent :type Primitive%20Component%20Object%20Reference) (OtherActor :type Actor%20Object%20Reference) (OtherComp :type Primitive%20Component%20Object%20Reference) (OtherBodyIndex :type Integer))
  (bind _asplayer_character (Utilities|Casting|CastToPlayerCharacter OtherActor))
  (if (Variables|Default|GetTowardsBoss)
    (Variables|Default|SetTowardsBoss false)
    (bind _extendspringarm (Timeline|SpringArmExtension PlayFromStart)
      (:Update
        (Variables|/Script/Engine.SpringArmComponent|SetTargetArmLength (Variables|/Game/Deadbit/Blueprints/ThirdPersonCharacter/PlayerCharacter.PlayerCharacter_C|GetSpringArm _asplayer_character) _extendspringarm)))))

(event OnComponentEndOverlap(Box)
  (params (OverlappedComponent :type Primitive%20Component%20Object%20Reference) (OtherActor :type Actor%20Object%20Reference) (OtherComp :type Primitive%20Component%20Object%20Reference) (OtherBodyIndex :type Integer))
  (Utilities|Casting|CastToPlayerCharacter OtherActor)
  (if (Variables|Default|GetAwayFromBoss)
    (Variables|Default|SetAwayFromBoss false)
    (bind _extendspringarm (Timeline|SpringArmExtension Reverse)
      (:Update
        (Variables|/Script/Engine.SpringArmComponent|SetTargetArmLength (Variables|/Game/Deadbit/Blueprints/ThirdPersonCharacter/PlayerCharacter.PlayerCharacter_C|GetSpringArm (stale OnComponentEndOverlap(Box2) _asplayer_character)) _extendspringarm)))))

(event OnComponentBeginOverlap(Box2)
  (params (OverlappedComponent :type Primitive%20Component%20Object%20Reference) (OtherActor :type Actor%20Object%20Reference) (OtherComp :type Primitive%20Component%20Object%20Reference) (OtherBodyIndex :type Integer) (bFromSweep :type Boolean) (SweepResult :type Hit%20Result%20Structure%20%28by%20ref%29))
  (Utilities|Casting|CastToPlayerCharacter OtherActor
    (:then
      (Variables|Default|SetAwayFromBoss true))
    (:CastFailed
      (Variables|Default|SetAwayFromBoss false))))

(fn ConstructionScript)