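; HealthPad is a healing pad that restores health to ModularRobots standing in its Box.
; Tick, throttled by a DoOnce and Delay, runs HealRobot on each overlapping robot, adding health up to its maximum.
; Each result swaps the active and inactive particle systems, so the last robot checked sets the look.
; Leaving the box switches off the robot's ParticleSystem; an older negative-damage healing loop remains unconnected.
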(event OnComponentBeginOverlap(Box)
  (params (OverlappedComponent :type Primitive%20Component%20Object%20Reference) (OtherActor :type Actor%20Object%20Reference) (OtherComp :type Primitive%20Component%20Object%20Reference) (OtherBodyIndex :type Integer) (bFromSweep :type Boolean) (SweepResult :type Hit%20Result%20Structure%20%28by%20ref%29)))

(event OnComponentEndOverlap(Box)
  (params (OverlappedComponent :type Primitive%20Component%20Object%20Reference) (OtherActor :type Actor%20Object%20Reference) (OtherComp :type Primitive%20Component%20Object%20Reference) (OtherBodyIndex :type Integer))
  (bind _asmodular_robot (Utilities|Casting|CastToModularRobot OtherActor))
  (Components|Activation|Deactivate (Variables|/Game/Deadbit/Blueprints/RobotParts/ModularRobot.ModularRobot_C|GetParticleSystem _asmodular_robot))
  (Rendering|SetVisibility (Variables|/Game/Deadbit/Blueprints/RobotParts/ModularRobot.ModularRobot_C|GetParticleSystem _asmodular_robot) false false))

(event EventTick
  (params (DeltaSeconds :type Float%20%28single-precision%29))
  (bind _activesystem (Variables|Default|GetActiveSystem))
  (bind _activesystem_2 (Variables|Default|GetActiveSystem))
  (bind _inactivesystem (Variables|Default|GetInactiveSystem))
  (bind _inactivesystem_2 (Variables|Default|GetInactiveSystem))
  (Utilities|FlowControl|DoOnce false :!label _label
    (:Completed
      (for _array_element (Collision|GetOverlappingActors (Variables|Default|GetBox) "/Game/Deadbit/Blueprints/RobotParts/ModularRobot.ModularRobot_C" :!class /Script/Engine.PrimitiveComponent)
        (bind _success (CallFunction|HealRobot (.AsModular%20Robot (Utilities|Casting|CastToModularRobot _array_element))))
        (if _success
          (Components|Activation|Activate _activesystem_2 true)
          (Rendering|SetVisibility _activesystem_2 true false)
          (Components|Activation|Deactivate _inactivesystem)
          (Rendering|SetVisibility _inactivesystem false false)
          (else
            (Components|Activation|Deactivate _activesystem)
            (Rendering|SetVisibility _activesystem false false)
            (Components|Activation|Activate _inactivesystem_2 true)
            (Rendering|SetVisibility _inactivesystem_2 true false))))
      (Utilities|FlowControl|Delay (Variables|Default|GetSeconds%20Between%20Ticks))
      (goto _label Reset))))

(fn ConstructionScript)

(fn HealRobot
  (params (Robot :type Modular%20Robot%20Object%20Reference))
  (if (< (Variables|/Game/Deadbit/Blueprints/Health/Health.Health_C|GetHealth (Variables|/Game/Deadbit/Blueprints/RobotParts/ModularRobot.ModularRobot_C|GetHealth Robot)) (Variables|/Game/Deadbit/Blueprints/Health/Health.Health_C|GetmaxHealth (Variables|/Game/Deadbit/Blueprints/RobotParts/ModularRobot.ModularRobot_C|GetHealth Robot)))
    (bind _output_get (Variables|/Game/Deadbit/Blueprints/Health/Health.Health_C|SetHealth (Variables|/Game/Deadbit/Blueprints/RobotParts/ModularRobot.ModularRobot_C|GetHealth Robot) (+ (Variables|/Game/Deadbit/Blueprints/Health/Health.Health_C|GetHealth (Variables|/Game/Deadbit/Blueprints/RobotParts/ModularRobot.ModularRobot_C|GetHealth Robot)) (Variables|Default|GetHealing%20Per%20Tick))))
    (if (> _output_get (Variables|/Game/Deadbit/Blueprints/Health/Health.Health_C|GetmaxHealth (Variables|/Game/Deadbit/Blueprints/RobotParts/ModularRobot.ModularRobot_C|GetHealth Robot)))
      (Variables|/Game/Deadbit/Blueprints/Health/Health.Health_C|SetHealth (Variables|/Game/Deadbit/Blueprints/RobotParts/ModularRobot.ModularRobot_C|GetHealth Robot) (Variables|/Game/Deadbit/Blueprints/Health/Health.Health_C|GetmaxHealth (Variables|/Game/Deadbit/Blueprints/RobotParts/ModularRobot.ModularRobot_C|GetHealth Robot))))
    (return true)
    (else
      (return false))))