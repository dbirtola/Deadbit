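; Sliding door that opens for overlapping pawns and can stay locked until a linked list of robots is killed.
; Robot death events count down to unlock it, and the trigger box rechecks living robots' factions before opening.
; A timeline slides the door with sounds and switches vision collision's object type, reversing shortly after the box empties.
; Construction picks boss or regular dynamic materials, whose parameters Lock and Unlock set to show state.
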(event OnComponentBeginOverlap(Box)
  (params (OverlappedComponent :type Primitive%20Component%20Object%20Reference) (OtherActor :type Actor%20Object%20Reference) (OtherComp :type Primitive%20Component%20Object%20Reference) (OtherBodyIndex :type Integer) (bFromSweep :type Boolean) (SweepResult :type Hit%20Result%20Structure%20%28by%20ref%29))
  (if (Variables|Default|GetLocked)
    (if (not (== 0 (Utilities|Array|Length (Variables|Default|GetrobotsToKill))))
      ;[1 1 1] lock door if at least one robot is alive, unlock if they are all dead.
      (bind _array_element (Utilities|Array|ForEachLoopwithBreak (Variables|Default|GetrobotsToKill) :!label _label)
        (:LoopBody
          (bind _alive (Default|IsAlive (Variables|/Game/Deadbit/Blueprints/RobotParts/ModularRobot.ModularRobot_C|GetHealth _array_element)))
          (if _alive
            (if (Utilities|Enum|Equal(Enum) (Variables|/Game/Deadbit/Blueprints/RobotParts/ModularRobot.ModularRobot_C|GetFaction _array_element) "NewEnumerator1")
              (Variables|Default|SetLocked true)
              (Variables|Default|SetLiveRobot true))
            (else
              (if (not (Variables|Default|GetLiveRobot)) :!label _label_2
                (Variables|Default|SetLiveRobot false)
                (CallFunction|Unlock)
                (Utilities|Casting|CastToPawn OtherActor)
                (Collision|SetCollisionObjectType (Variables|Default|GetVisionCollision) "ECC_WorldDynamic")
                (Audio|PlaySoundatLocation "/Game/Deadbit/Sound/SoundCues/DoorOpen.DoorOpen" (Transformation|GetActorLocation) "0, 0, 0" 1.0 1.0 0.0 0 0 0)
                (bind _movement (Timeline|Timeline_0 Play)
                  (:Update
                    (Transformation|SetRelativeLocation (Variables|Default|GetDoor) (Math|Vector|Lerp(Vector) "0, 0,-230.000000" "0, 0, 0" _movement) false false)))))))
        (:Completed
          (goto _label_2))))
    (else
      (goto _label))))

(event OnComponentEndOverlap(Box)
  (params (OverlappedComponent :type Primitive%20Component%20Object%20Reference) (OtherActor :type Actor%20Object%20Reference) (OtherComp :type Primitive%20Component%20Object%20Reference) (OtherBodyIndex :type Integer))
  (Variables|Default|SetLiveRobot false)
  (Utilities|Casting|CastToPawn OtherActor)
  (Utilities|FlowControl|Delay 1.0)
  (if (== (Utilities|Array|Length (Collision|GetOverlappingActors (Variables|Default|GetBox) "/Script/Engine.Pawn" :!class /Script/Engine.PrimitiveComponent)) 0)
    (Audio|PlaySoundatLocation "/Game/Deadbit/Sound/SoundCues/DoorClosed.DoorClosed" (Transformation|GetActorLocation) "0, 0, 0" 1.0 1.0 0.0 0 0 0)
    (Collision|SetCollisionObjectType (Variables|Default|GetVisionCollision) "ECC_WorldStatic")
    (bind _movement (Timeline|Timeline_0 Reverse)
      (:Update
        (Transformation|SetRelativeLocation (Variables|Default|GetDoor) (Math|Vector|Lerp(Vector) "0, 0,-230.000000" "0, 0, 0" _movement) false false)))))

(event Custom|DecrementRemaining
  (bind _output_get (Variables|Default|SetRobotsRemaining (Utilities|-- (Variables|Default|GetRobotsRemaining))))
  (if (<= _output_get 0)
    (CallFunction|UnlockDoor)))

(event Custom|UnlockDoor
  (CallFunction|Unlock))

(event EventBeginPlay
  (bind _robotstokill (Variables|Default|GetrobotsToKill))
  (bind _returnvalue (Utilities|Array|Length _robotstokill))
  (bind _returnvalue_2 (== 0 _returnvalue))
  (if (Variables|Default|GetLocked)
    (if _returnvalue_2 ; If the door starts locked but there are bots to kill, bind opening event to their deaths
      (CallFunction|Lock :!label _label)
      (else
        (Variables|Default|SetRobotsRemaining _returnvalue :!label _label_2)
        (for _array_element (Variables|Default|GetrobotsToKill)
          (EventDispatchers|BindEventtoDeath (Variables|/Game/Deadbit/Blueprints/RobotParts/ModularRobot.ModularRobot_C|GetHealth _array_element) (delegate Custom|DecrementRemaining)))
        (Variables|Default|SetLocked true)
        (if (Variables|Default|GetLocked)
          (goto _label)
          (else
            (CallFunction|Unlock)))))
    (elif (not _returnvalue_2)
      (goto _label_2))))

(fn ConstructionScript
  (if (Variables|Default|GetIsBossDoor)
    (bind _returnvalue (Rendering|Material|CreateDynamicMaterialInstance (Variables|Default|GetPlane) 0 "/Game/Deadbit/Materials/M_DoorBarrier_Inst2.M_DoorBarrier_Inst2" "None" :!class /Script/Engine.PrimitiveComponent))
    (Variables|Default|SetMaterial-Door _returnvalue)
    (bind _returnvalue_2 (Rendering|Material|CreateDynamicMaterialInstance (Variables|Default|GetDoor) 0 "/Game/Deadbit/3D/Props/Door/M_Prop_DoorDoor_Inst2.M_Prop_DoorDoor_Inst2" "None" :!class /Script/Engine.PrimitiveComponent))
    (Variables|Default|SetMaterial-Arrows _returnvalue_2)
    (else
      (bind _returnvalue_3 (Rendering|Material|CreateDynamicMaterialInstance (Variables|Default|GetPlane) 0 "/Game/Deadbit/Materials/M_DoorBarrier_Inst.M_DoorBarrier_Inst" "None" :!class /Script/Engine.PrimitiveComponent))
      (Variables|Default|SetMaterial-Door _returnvalue_3)
      (bind _returnvalue_4 (Rendering|Material|CreateDynamicMaterialInstance (Variables|Default|GetDoor) 0 "/Game/Deadbit/3D/Props/Door/M_Prop_DoorDoor_Inst1.M_Prop_DoorDoor_Inst1" "None" :!class /Script/Engine.PrimitiveComponent))
      (Variables|Default|SetMaterial-Arrows _returnvalue_4))))

(fn Lock
  (Variables|Default|SetLocked true)
  (Rendering|Material|SetScalarParameterValue (Variables|Default|GetMaterial-Arrows) "DoorLocked?" 1.0 :!class /Script/Engine.MaterialInstanceDynamic)
  (Rendering|Material|SetScalarParameterValue (Variables|Default|GetMaterial-Door) "LowHealth" 1.0 :!class /Script/Engine.MaterialInstanceDynamic))

(fn Unlock
  (Variables|Default|SetLocked false)
  (Rendering|Material|SetScalarParameterValue (Variables|Default|GetMaterial-Arrows) "DoorLocked?" 0.0 :!class /Script/Engine.MaterialInstanceDynamic)
  (Rendering|Material|SetScalarParameterValue (Variables|Default|GetMaterial-Door) "LowHealth" 0.0 :!class /Script/Engine.MaterialInstanceDynamic))