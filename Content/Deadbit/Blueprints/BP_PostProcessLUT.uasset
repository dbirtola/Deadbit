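; BP_PostProcessLUT is an actor that cycles its post process through a list of LUTs, apparently for previewing color grading looks.
; On BeginPlay it starts a looping timer with a configurable delay.
; Each timer tick advances a wrapping index, rebuilds the post-process settings from the selected LUT and prints that LUT's name on screen.
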(event Custom|CycleLUT'S
  (bind _lut_stocyclethrough (Variables|Cycling|GetLUT'sToCycleThrough))
  (bind _result (Math|Integer|IncrementInt (Variables|Cycling|GetCycleIndex))
    (:%20%20
      (bind _output_get (Variables|Cycling|SetCycleIndex (Math|Integer|%(Integer) _result (Utilities|Array|Length _lut_stocyclethrough))))
      (Variables|/Script/Engine.PostProcessComponent|SetSettings (Variables|Default|GetPostProcess) (Utilities|Struct|MakePostProcessSettings (Utilities|Array|Get(acopy) _lut_stocyclethrough _output_get)))
      (Development|PrintString (Utilities|GetObjectName (Utilities|Array|Get(acopy) _lut_stocyclethrough _output_get))))))

(event EventBeginPlay
  (Utilities|Time|SetTimerbyEvent (delegate Custom|CycleLUT'S) (Variables|Cycling|GetCycleDelay) true))

(event Collision|EventActorBeginOverlap
  (params (OtherActor :type Actor%20Object%20Reference)))

(event EventTick
  (params (DeltaSeconds :type Float%20%28single-precision%29)))

(fn ConstructionScript)