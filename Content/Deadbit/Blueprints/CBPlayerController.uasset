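; Player controller that creates the HUD and handles robot and part interaction for the player.
; On BeginPlay it finds the first BasicBot and sets the controlled pawn as its owner.
; R uses the character's interaction collider to pick up robot parts into a hidden owned list or toggle the HUD's robot editor for modular robots.
; Debug keys send the bot a damage event or toggle its event-queue display.
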(event EventBeginPlay
  (bind _returnvalue (UserInterface|CreateWidget "/Game/Deadbit/Blueprints/UMG/HUD.HUD_C"))
  (UserInterface|Viewport|AddtoViewport _returnvalue 0)
  (Variables|Default|SetHUD _returnvalue)
  (bind _outactors (Actor|GetAllActorsOfClass "/Game/Deadbit/Blueprints/RobotParts/Cores/BasicBot.BasicBot_C"))
  (Variables|Default|SetRobot (Utilities|Array|Get(acopy) _outactors))
  (Actor|SetOwner (Utilities|Array|Get(acopy) _outactors) (Pawn|GetControlledPawn)))

(event Input|KeyboardEvents|R
  (params (Key :type Key%20Structure))
  (bind _returnvalue (Pawn|GetControlledPawn))
  (bind _asthird_person_character (Utilities|Casting|CastToThirdPersonCharacter _returnvalue))
  (bind _interactioncollider (Variables|/Game/Deadbit/Blueprints/ThirdPersonCharacter.ThirdPersonCharacter_C|GetInteractionCollider _asthird_person_character))
  (bind _overlappingactors (Collision|GetOverlappingActors _interactioncollider "/Game/Deadbit/Blueprints/RobotParts/ModularRobot.ModularRobot_C" :!class /Script/Engine.PrimitiveComponent))
  (bind _output (Utilities|Array|Get(acopy) _overlappingactors))
  (:Pressed
    (Utilities|IsValid _output
      (:Is%20Valid
        (Default|ToggleRobotEditor (Variables|Default|GetHUD) (.AsModular%20Robot (Utilities|Casting|CastToModularRobot _output)))))))

(event Input|KeyboardEvents|T
  (params (Key :type Key%20Structure))
  (:Pressed
    (Default|ToggleDebug (Variables|Default|GetHUD) (Variables|/Game/Deadbit/Blueprints/RobotParts/ModularRobot.ModularRobot_C|GetEventQueue (Variables|Default|GetRobot)))))

(event Input|MouseEvents|LeftMouseButton
  (params (Key :type Key%20Structure))
  (:Pressed
    (if (Variables|Default|GetbShowMouseCursor)
      (Audio|PlaySound2D "/Game/Deadbit/Sound/SoundCues/UIClick.UIClick" 1.0 1.0 0.0 0 0))))

(event Input|KeyboardEvents|R
  (params (Key :type Key%20Structure))
  (bind _returnvalue (Pawn|GetControlledPawn))
  (bind _asthird_person_character (Utilities|Casting|CastToThirdPersonCharacter _returnvalue))
  (bind _interactioncollider (Variables|/Game/Deadbit/Blueprints/ThirdPersonCharacter.ThirdPersonCharacter_C|GetInteractionCollider _asthird_person_character))
  (bind _overlappingactors (Collision|GetOverlappingActors _interactioncollider "/Game/Deadbit/Blueprints/RobotParts/RobotPart.RobotPart_C" :!class /Script/Engine.PrimitiveComponent))
  (bind _output (Utilities|Array|Get(acopy) _overlappingactors))
  (:Pressed
    (Utilities|IsValid _output
      (:Is%20Valid
        (bind _asrobot_part (Utilities|Casting|CastToRobotPart _output))
        (CallFunction|PickupPart _asrobot_part)))))

(event Input|KeyboardEvents|E
  (params (Key :type Key%20Structure))
  (:Pressed
    (Default|TakeDamageEvent (Variables|Default|GetRobot))))

(fn ConstructionScript)

(fn PickupPart
  (params (Part :type Robot%20Part%20Object%20Reference))
  (Utilities|IsValid Part
    (:Is%20Valid
      (Utilities|Array|Add (Variables|Default|GetOwnedParts) Part)
      (Rendering|SetVisibility (Variables|/Game/Deadbit/Blueprints/RobotParts/RobotPart.RobotPart_C|GetDefaultSceneRoot Part) false true))))

(fn RemovePart
  (params (Robot%20Part :type Robot%20Part%20Object%20Reference))
  (Utilities|Array|RemoveItem (Variables|Default|GetOwnedParts) Robot%20Part))