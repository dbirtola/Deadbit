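; Sliding door actor that stays locked while robots of a given faction in its RobotsToKill list are alive.
; BeginPlay locks it if that list is populated, and a scalar material parameter on the door reflects lock state.
; Box overlap rechecks robot health, then, if clear, plays a sound and a timeline lerping the door's relative location for pawns.
; When the player leaves, it reverses the timeline after a short delay.
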(event OnComponentBeginOverlap(Box)
  (params (OverlappedComponent :type Primitive%20Component%20Object%20Reference) (OtherActor :type Actor%20Object%20Reference) (OtherComp :type Primitive%20Component%20Object%20Reference) (OtherBodyIndex :type Integer) (bFromSweep :type Boolean) (SweepResult :type Hit%20Result%20Structure%20%28by%20ref%29))
  ;[1 1 1] lock door if at least one robot is alive, unlock if they are all dead.
  (bind _array_element (Utilities|Array|ForEachLoopwithBreak (Variables|Default|GetrobotsToKill))
    (:LoopBody
      (bind _alive (Default|IsAlive (Variables|/Game/Deadbit/Blueprints/RobotParts/ModularRobot.ModularRobot_C|GetHealth _array_element)))
      (if _alive
        (if (Utilities|Enum|Equal(Enum) (Variables|/Game/Deadbit/Blueprints/RobotParts/ModularRobot.ModularRobot_C|GetFaction _array_element) "NewEnumerator1")
          (Variables|Default|SetLocked true)
          (Variables|Default|SetLiveRobot true))
        (else
          (if (Variables|Default|GetLiveRobot) :!label _label
            (Rendering|Material|SetScalarParameterValueonMaterials (Variables|Default|GetDoor) "DoorLocked" 0.0)
            (else
              (Variables|Default|SetLocked false)
              (Variables|Default|SetLiveRobot false)
              (Rendering|Material|SetScalarParameterValueonMaterials (Variables|Default|GetDoor) "DoorLocked" 1.0)
              (Utilities|Casting|CastToPawn OtherActor)
              (Audio|PlaySoundatLocation "/Game/Deadbit/Sound/SoundCues/DoorOpen.DoorOpen" "0, 0, 0" "0, 0, 0" 1.0 1.0 0.0 0 0 0)
              (bind _movement (Timeline|Timeline_1 Play)
                (:Update
                  (Transformation|SetRelativeLocation (Variables|Default|GetDoor) (Math|Vector|Lerp(Vector) "0, 0,250.000000" "0, 0, 0" _movement) false false))))))))
    (:Completed
      (goto _label))))

(event OnComponentEndOverlap(Box)
  (params (OverlappedComponent :type Primitive%20Component%20Object%20Reference) (OtherActor :type Actor%20Object%20Reference) (OtherComp :type Primitive%20Component%20Object%20Reference) (OtherBodyIndex :type Integer))
  (Variables|Default|SetLiveRobot false)
  (Utilities|Casting|CastToPlayerCharacter OtherActor)
  (Utilities|FlowControl|Delay 1.0)
  (Audio|PlaySoundatLocation "/Game/Deadbit/Sound/SoundCues/DoorClosed.DoorClosed" "0, 0, 0" "0, 0, 0" 1.0 1.0 0.0 0 0 0)
  (bind _movement (Timeline|Timeline_1 Reverse)
    (:Update
      (Transformation|SetRelativeLocation (Variables|Default|GetDoor) (Math|Vector|Lerp(Vector) "0, 0,250.000000" "0, 0, 0" _movement) false false))))

(event Custom|CustomEvent
  (params (OverlappedComponent :type Primitive%20Component%20Object%20Reference) (OtherActor :type Actor%20Object%20Reference) (OtherComp :type Primitive%20Component%20Object%20Reference) (OtherBodyIndex :type Integer) (bFromSweep :type Boolean) (SweepResult :type Hit%20Result%20Structure%20%28by%20ref%29)))

(event Custom|CustomEvent_1
  (params (OverlappedComponent :type Primitive%20Component%20Object%20Reference) (OtherActor :type Actor%20Object%20Reference) (OtherComp :type Primitive%20Component%20Object%20Reference) (OtherBodyIndex :type Integer)))

(event EventBeginPlay
  (if (not (== 0.0 (Math|Conversions|ToFloat(Integer) (Utilities|Array|Length (Variables|Default|GetrobotsToKill)))))
    (Variables|Default|SetLocked true)
    (if (Variables|Default|GetLocked)
      (bind _returnvalue (Rendering|Material|CreateDynamicMaterialInstance (Variables|Default|GetDoor) 0 "/Game/Deadbit/3D/Props/Door/oldDoor/M_Door_Inst.M_Door_Inst" "None" :!class /Script/Engine.PrimitiveComponent))
      (Rendering|Material|SetScalarParameterValue _returnvalue "DoorLocked?" 1.0 :!class /Script/Engine.MaterialInstanceDynamic)
      (else
        (Rendering|Material|SetScalarParameterValueonMaterials (Variables|Default|GetDoor) "DoorLocked?" 1.0)))))

(event EventTick
  (params (DeltaSeconds :type Float%20%28single-precision%29)))

(event Collision|EventActorBeginOverlap
  (params (OtherActor :type Actor%20Object%20Reference)))

(fn ConstructionScript)