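; Game mode that starts a level, loads saved progress when requested, and restarts on player death.
; On BeginPlay, a "?Load" options string makes it fire LoadGameEvent on the GameManager actor.
; It also binds RestartGame to the player character's Health death event.
; RestartGame reopens the hardcoded Tutorial_John2 level with the Load option, so death returns the player to the saved game.
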(event Custom|Restart%20Game
  (Development|PrintString "Zoe DIED!")
  (Game|OpenLevel(byName) "Tutorial_John2" true "Load"))

(event EventBeginPlay
  (bind _optionsstring (Variables|Default|GetOptionsString))
  (Utilities|FlowControl|Sequence
    (:then_0
      (Development|PrintString _optionsstring)
      (if (Utilities|Enum|Equal(Enum) _optionsstring "?Load")
        (Development|PrintString "Loading Game")
        (bind _outactors (Actor|GetAllActorsOfClass "/Game/Deadbit/Blueprints/GameManager.GameManager_C"))
        (Default|LoadGameEvent (Utilities|Array|Get(acopy) _outactors))
        (else
          (Development|PrintString "Not Loading Game"))))
    (:then_1
      (bind _asplayer_character (Utilities|Casting|CastToPlayerCharacter (Game|Player|GetPlayerPawn 0)))
      (EventDispatchers|BindEventtoDeath (Variables|/Game/Deadbit/Blueprints/ThirdPersonCharacter/PlayerCharacter.PlayerCharacter_C|GetHealth _asplayer_character) (delegate Custom|Restart%20Game)))))

(fn ConstructionScript)