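; Base tutorial step object that sequences tutorial steps from a data table, with child classes meant to override StartStep.
; Begin stores the table and row position, looks up the row's named actor as NextStep, then calls StartStep and prints a debug string.
; StartStep defaults to calling FinishStep immediately, which calls Begin again with the stored table state.
; The chain stops when rows run out or the actor cast fails.
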(event Custom|Begin
  (params (TutorialTable :type Data%20Table%20Object%20Reference) (RowNames :type Array%20of%20Names) (NextRowNum :type Integer))
  (Variables|Default|SetTutorial%20Table TutorialTable)
  (bind _output_get (Variables|Default|SetRow%20Names RowNames))
  (bind _output_get_2 (Variables|Default|SetNextRowNum NextRowNum))
  (if (< _output_get_2 (Utilities|Array|Length _output_get))
    (bind _tutorial_actor (CallFunction|BreakTutorialRow (Variables|Default|GetTutorial%20Table) (Variables|Default|GetRow%20Names) (Variables|Default|GetNextRowNum)))
    (bind _newparam (CallFunction|GetActorbyString _tutorial_actor "TutorialStepObj_C"))
    (bind _astutorial_step_obj (Utilities|Casting|CastToTutorialStepObj _newparam))
    (Variables|Default|SetNextStep _astutorial_step_obj)
    (CallFunction|StartStep)
    (Development|PrintString "oof")))

(event Custom|StartStep
  ;[1 1 1] Override this in child classes
  (CallFunction|FinishStep))

(event Custom|FinishStep
  ;[1 1 1] Connect to this at the end
  (CallFunction|Begin (Variables|Default|GetTutorial%20Table) (Variables|Default|GetRow%20Names) (Utilities|++ (Variables|Default|GetNextRowNum))))

(fn ConstructionScript)

(fn BreakTutorialRow
  (params (Tutorial%20Table :type Data%20Table%20Object%20Reference) (Row%20Names :type Array%20of%20Names) (Row%20Index :type Integer))
  (bind _output (Utilities|Array|Get(acopy) Row%20Names Row%20Index))
  (bind _returnvalue (Utilities|GetDataTableRow Tutorial%20Table _output)
    (:then
      (return (.Prompt (Utilities|Struct|BreakTutorialStep _returnvalue)) (.TutorialActor (Utilities|Struct|BreakTutorialStep _returnvalue))))
    (:RowNotFound
      (Development|PrintString (Utilities|String|Append "Row " (Utilities|String|ToString(Name) _output) " not found")))))