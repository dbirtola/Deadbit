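; Breakable vent that shakes when damaged, then notifies through CallDestroySelf and destroys itself when health runs out.
; While the player overlaps PunchBox, Tick moves PlayerTracker to the player's position so its local Y sign steers the first shake away from them.
; Shake nudges the mesh each frame via a zero-delay loop, reversing at a limit until it nears its start.
; Older in-vent punch detection remains disconnected.
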(event OnComponentBeginOverlap(PunchBox)
  (params (OverlappedComponent :type Primitive%20Component%20Object%20Reference) (OtherActor :type Actor%20Object%20Reference) (OtherComp :type Primitive%20Component%20Object%20Reference) (OtherBodyIndex :type Integer) (bFromSweep :type Boolean) (SweepResult :type Hit%20Result%20Structure%20%28by%20ref%29))
  (bind _asplayer_character (Utilities|Casting|CastToPlayerCharacter OtherActor))
  (Variables|Default|SetOverlapping true)
  (Variables|Default|SetPlayerLocation (Variables|/Script/Engine.Actor|GetRootComponent _asplayer_character)))

(event OnComponentEndOverlap(PunchBox)
  (params (OverlappedComponent :type Primitive%20Component%20Object%20Reference) (OtherActor :type Actor%20Object%20Reference) (OtherComp :type Primitive%20Component%20Object%20Reference) (OtherBodyIndex :type Integer))
  (Utilities|Casting|CastToPlayerCharacter OtherActor)
  (Variables|Default|SetOverlapping false))

(event Custom|DestroySelf_Event)

(event Custom|Shake
  (bind _staticmesh (Variables|Default|GetStaticMesh))
  (bind _relativelocation (Variables|/Script/Engine.SceneComponent|GetRelativeLocation _staticmesh))
  (bind (_x _y _z) (Math|Vector|BreakVector _relativelocation))
  (Variables|Default|SetShakeDirection (* (Utilities|GetSign (.Y (Math|Vector|BreakVector (Variables|/Script/Engine.SceneComponent|GetRelativeLocation (Variables|Default|GetPlayerTracker))))) (* (Variables|Default|GetShakeSpeed) -1.0)))
  (Utilities|FlowControl|Delay 0.0 :!label _label)
  (Transformation|SetRelativeLocation (Variables|Default|GetStaticMesh) (Math|Vector|MakeVector _x (+ _y (Variables|Default|GetShakeDirection)) _z) false false)
  (if (Math|Float|NearlyEqual(Float) (+ _y (Variables|Default|GetShakeDirection)) (* (Variables|Default|GetShakeLimit) (Variables|Default|GetShakeDirection)) 1.0)
    (Variables|Default|SetShakeDirection (* (Variables|Default|GetShakeDirection) -1.0)))
  (if (not (Math|Float|NearlyEqual(Float) (Variables|Default|GetInitialY) (+ _y (Variables|Default|GetShakeDirection)) 0.1))
    (goto _label)))

(event Custom|CustomEvent
  (params (DeltaSeconds :type Float%20%28single-precision%29)))

(event EventTick
  (params (DeltaSeconds :type Float%20%28single-precision%29))
  (if (Variables|Default|GetOverlapping)
    (Transformation|SetWorldLocation (Variables|Default|GetPlayerTracker) (Transformation|GetWorldLocation (Variables|Default|GetPlayerLocation)) false false)))

(event Game|Damage|EventAnyDamage
  (params (Damage :type Float%20%28single-precision%29) (DamageType :type Damage%20Type%20Object%20Reference) (InstigatedBy :type Controller%20Object%20Reference) (DamageCauser :type Actor%20Object%20Reference))
  (bind _output_get (Variables|Default|SetHealth (- (Variables|Default|GetHealth) Damage)))
  (CallFunction|Shake)
  (if (<= _output_get 0.0)
    (Default|CallDestroySelf)
    (Actor|DestroyActor)))

(event EventBeginPlay
  (Variables|Default|SetHealth (Variables|Default|GetMaxHealth))
  (Variables|Default|SetInitialY 0.0))

(fn ConstructionScript)