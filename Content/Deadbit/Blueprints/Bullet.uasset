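; Bullet is a projectile Blueprint that damages what it hits.
; When its Sphere component hits an actor other than its owner, it applies fixed damage credited to the owner's instigator controller.
; It then spawns an impact particle effect at the hit location, oriented along the surface normal, and destroys itself.
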(event OnComponentHit(Sphere)
  (params (HitComponent :type Primitive%20Component%20Object%20Reference) (OtherActor :type Actor%20Object%20Reference) (OtherComp :type Primitive%20Component%20Object%20Reference) (NormalImpulse :type Vector :default "0, 0, 0") (Hit :type Hit%20Result%20Structure%20%28by%20ref%29))
  (bind (_bblockinghit _binitialoverlap _time _distance _location _impactpoint _normal _impactnormal) (Collision|BreakHitResult Hit))
  (if (not (== OtherActor (Components|GetOwner)))
    (Game|Damage|ApplyDamage OtherActor 3e+01 (Game|GetInstigatorController (Components|GetOwner)) self)
    (Effects|SpawnEmitteratLocation "/Game/Deadbit/Cascade/P_Bullet_Impact.P_Bullet_Impact" _location (Math|Conversions|RotationFromXVector _impactnormal))
    (Actor|DestroyActor)))

(fn ConstructionScript)