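; PlayerLibrary holds health functions for the player: TakeDamage and Death.
; TakeDamage takes a Damage input, but its entry is unwired, so calling it does nothing.
; Its disconnected nodes cast player 0 to PlayerCharacter, call PlayerDamaged, set Health without a wired value, and call Death at zero or below.
; Death only prints a death message.
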(fn TakeDamage
  (params (damage :type Integer)))

(fn Death
  (Development|PrintString 0 "You are DEAD"))