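; Chip is a placeable grid actor that represents one CodePiece instruction in ChipStudio's visual programming board.
; It stores grid position and rotation on the CodePiece, displays it through a ChipWidget, and spawns notch meshes as connectors.
; Connect recursively links NextInstructions, finding the right neighbor by collision overlap and lower and upper ones by grid lookup.
; Parameter edits refresh the widget and make ChipStudio recreate the program.
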(event Custom|InitializeChip
  (params (Code%20Piece :type Code%20Piece%20Object%20Reference) (GridX :type Integer) (GridY :type Integer) (Rotation :type Direction%20Enum :default "NewEnumerator0"))
  (Variables|Default|SetGridX GridX)
  (Variables|Default|SetGridY GridY)
  (Variables|Default|SetRotation Rotation)
  (Utilities|Array|Resize (Variables|Default|GetNextChips) (Variables|/Game/Deadbit/Blueprints/BotProgramming/Functions/BaseClasses/CodePiece.CodePiece_C|GetMaxInstructions Code%20Piece))
  (bind _output_get (Variables|Default|SetCodePiece Code%20Piece))
  (Variables|/Game/Deadbit/Blueprints/BotProgramming/Functions/BaseClasses/CodePiece.CodePiece_C|SetGridX (Variables|Default|GetCodePiece) (Variables|Default|GetGridX))
  (Variables|/Game/Deadbit/Blueprints/BotProgramming/Functions/BaseClasses/CodePiece.CodePiece_C|SetGridY (Variables|Default|GetCodePiece) (Variables|Default|GetGridY))
  (Variables|/Game/Deadbit/Blueprints/BotProgramming/Functions/BaseClasses/CodePiece.CodePiece_C|SetRotation (Variables|Default|GetCodePiece) (Variables|Default|GetRotation))
  (Default|Refresh (.AsChip%20Widget (Utilities|Casting|CastToChipWidget (UserInterface|GetUserWidgetObject (Variables|Default|GetWidget)))) _output_get self)
  (CallFunction|CreateConnectors))

(event Custom|Set%20Parameter%20By%20Index
  (params (Index :type Integer) (Parameter%20Piece :type Code%20Piece%20Object%20Reference))
  (bind _codepiece (Variables|Default|GetCodePiece))
  (Variables|/Game/Deadbit/Blueprints/BotProgramming/Functions/BaseClasses/CodePiece.CodePiece_C|SetProgram Parameter%20Piece (Variables|/Game/Deadbit/Blueprints/BotProgramming/Functions/BaseClasses/CodePiece.CodePiece_C|GetProgram _codepiece))
  (Utilities|Array|SetArrayElem (Variables|/Game/Deadbit/Blueprints/BotProgramming/Functions/BaseClasses/CodePiece.CodePiece_C|GetParameters _codepiece) 0 Parameter%20Piece)
  (bind _aschip_widget (Utilities|Casting|CastToChipWidget (UserInterface|GetUserWidgetObject (Variables|Default|GetWidget))))
  (Default|Refresh _aschip_widget (Variables|Default|GetCodePiece) self)
  (Default|CreateProgram (Variables|Default|GetChipStudio)))

(event Custom|Connect
  (params (Program :type Program%20Object%20Reference))
  (bind _codepiece (Variables|Default|GetCodePiece))
  (bind _codepiece_2 (Variables|Default|GetCodePiece))
  (bind _codepiece_3 (Variables|Default|GetCodePiece))
  (bind _nextinstructions (Variables|/Game/Deadbit/Blueprints/BotProgramming/Functions/BaseClasses/CodePiece.CodePiece_C|GetNextInstructions _codepiece))
  (bind _nextinstructions_2 (Variables|/Game/Deadbit/Blueprints/BotProgramming/Functions/BaseClasses/CodePiece.CodePiece_C|GetNextInstructions _codepiece_2))
  (bind _nextinstructions_3 (Variables|/Game/Deadbit/Blueprints/BotProgramming/Functions/BaseClasses/CodePiece.CodePiece_C|GetNextInstructions _codepiece_3))
  (bind _output_get (Variables|Default|SetProgram Program))
  (Variables|/Game/Deadbit/Blueprints/BotProgramming/Functions/BaseClasses/CodePiece.CodePiece_C|SetProgram (Variables|Default|GetCodePiece) _output_get)
  (Utilities|FlowControl|Sequence
    (:then_0
      ;[1 1 1] If we need 1 instruction
      (if (> (Variables|/Game/Deadbit/Blueprints/BotProgramming/Functions/BaseClasses/CodePiece.CodePiece_C|GetMaxInstructions (Variables|Default|GetCodePiece)) 0)
        ;[1 1 1] Get the chip to the right.
        (bind _aschip (Utilities|Casting|CastToChip (Utilities|Array|Get(acopy) (Collision|GetOverlappingActors (Variables|Default|GetRightConnectorCollision) "Chip_C" :!class /Script/Engine.PrimitiveComponent)))
          (:then
            (bind _output_get_2 (Variables|Default|SetRightChip _aschip))
            (CallFunction|Connect _output_get_2 (Variables|Default|GetProgram))
            ;[1 1 1] Set the next instruction to be code piece to the right
            (Utilities|IsValid (Variables|Default|GetRightChip)
              (:Is%20Valid
                (Utilities|Array|SetArrayElem _nextinstructions_3 0 (Variables|Chip_C|GetCodePiece (Variables|Default|GetRightChip)))
                ;[1 1 1] If we need 2 instruction
                (if (> (Variables|/Game/Deadbit/Blueprints/BotProgramming/Functions/BaseClasses/CodePiece.CodePiece_C|GetMaxInstructions (Variables|Default|GetCodePiece)) 1)
                  ;[1 1 1] Get the chip bellow.
                  (bind _chip (Default|GetChipatLocation (Variables|Default|GetChipStudio) (Variables|Default|GetGridX) (+ (Variables|Default|GetGridY) 1)))
                  ;[1 1 1] Set the next instruction to be code piece below
                  (CallFunction|Connect _chip (Variables|Default|GetProgram))
                  (Utilities|IsValid _chip
                    (:Is%20Valid
                      (Utilities|Array|SetArrayElem _nextinstructions_2 1 (Variables|Chip_C|GetCodePiece _chip))
                      ;[1 1 1] If we need 3 instruction
                      (if (> (Variables|/Game/Deadbit/Blueprints/BotProgramming/Functions/BaseClasses/CodePiece.CodePiece_C|GetMaxInstructions (Variables|Default|GetCodePiece)) 2)
                        ;[1 1 1] Get the chip above.
                        (bind _chip_2 (Default|GetChipatLocation (Variables|Default|GetChipStudio) (Variables|Default|GetGridX) (- (Variables|Default|GetGridY) 1)))
                        (CallFunction|Connect _chip_2 (Variables|Default|GetProgram))
                        ;[1 1 1] Set the next instruction to be code piece above
                        (Utilities|IsValid _chip_2
                          (:Is%20Valid
                            (Utilities|Array|SetArrayElem _nextinstructions 2 (Variables|Chip_C|GetCodePiece _chip_2)))
                          (:Is%20Not%20Valid
                            (Utilities|Array|SetArrayElem _nextinstructions 2 0)))))
                    (:Is%20Not%20Valid
                      (Utilities|Array|SetArrayElem _nextinstructions_2 1 0)))))
              (:Is%20Not%20Valid
                (Utilities|Array|SetArrayElem _nextinstructions_3 0 0))))
          (:CastFailed
            (Utilities|Array|SetArrayElem (Variables|/Game/Deadbit/Blueprints/BotProgramming/Functions/BaseClasses/CodePiece.CodePiece_C|GetNextInstructions (Variables|Default|GetCodePiece)) 0 0)))))
    (:then_1
      (for _array_element (Variables|/Game/Deadbit/Blueprints/BotProgramming/Functions/BaseClasses/CodePiece.CodePiece_C|GetParameters (Variables|Default|GetCodePiece))
        (Variables|/Game/Deadbit/Blueprints/BotProgramming/Functions/BaseClasses/CodePiece.CodePiece_C|SetProgram _array_element (Variables|Default|GetProgram))))))

(event Custom|CreateConnectors
  (bind _rightconnector (Variables|Default|GetRightConnector))
  ;[1 1 1] Create the first connector and set the location and rotation
  (if (>= (Variables|/Game/Deadbit/Blueprints/BotProgramming/Functions/BaseClasses/CodePiece.CodePiece_C|GetMaxInstructions (Variables|Default|GetCodePiece)) 1)
    (bind _returnvalue (AddComponent|AddStaticMeshComponent self false (Math|Transform|MakeTransform "0, 0, 0" (Variables|/Script/Engine.SceneComponent|GetRelativeRotation _rightconnector) "1,1,1")))
    (Transformation|SetWorldLocation _returnvalue (Transformation|GetWorldLocation _rightconnector) false false)
    (Components|StaticMesh|SetStaticMesh _returnvalue "/Game/Deadbit/Meshes/Chip_Notch_01.Chip_Notch_01")
    (Transformation|SetRelativeScale3D _returnvalue (Variables|/Script/Engine.SceneComponent|GetRelativeScale3D (Variables|Default|GetStaticMesh)))
    ;[1 1 1] Second connector, can just copy and paste but not sure if I like how the first connector is being set yet
    (if (>= (Variables|/Game/Deadbit/Blueprints/BotProgramming/Functions/BaseClasses/CodePiece.CodePiece_C|GetMaxInstructions (Variables|Default|GetCodePiece)) 2)
      (bind _returnvalue_2 (AddComponent|AddStaticMeshComponent self false (Transformation|GetRelativeTransform (Variables|Default|GetBottomConnector))))
      (Components|StaticMesh|SetStaticMesh _returnvalue_2 "/Game/Deadbit/Meshes/Chip_Notch_01.Chip_Notch_01"))))

(event Custom|Rotate
  (bind _output_get (Variables|Default|SetRotation (Utilities|Enum|ByteToEnumDirection (+ (Variables|Default|GetRotation) 1))))
  (if (> _output_get 3)
    (Variables|Default|SetRotation "NewEnumerator0"))
  (Development|PrintString (Utilities|String|Append "Rotation is now: " (Utilities|String|EnumtoString (Variables|Default|GetRotation))))
  (Transformation|SetWorldRotation (Variables|Default|GetScene) (Math|Rotator|MakeRotator 0.0 0.0 (* (Math|Conversions|ToInteger(Byte) (Variables|Default|GetRotation)) 9e+01)) false false)
  (Transformation|SetWorldRotation (Variables|Default|GetWidget) (Math|Rotator|MakeRotator 0.0 9e+01 1.8e+02) false false)
  (Variables|/Game/Deadbit/Blueprints/BotProgramming/Functions/BaseClasses/CodePiece.CodePiece_C|SetRotation (Variables|Default|GetCodePiece) (Variables|Default|GetRotation)))

(event EventBeginPlay
  (bind _outactors (Actor|GetAllActorsOfClass "/Game/Deadbit/Blueprints/UMG/ChipStudio.ChipStudio_C"))
  (Variables|Default|SetChipStudio (Utilities|Array|Get(acopy) _outactors)))

(fn ConstructionScript)

(fn GetCodePiece
  (return (Variables|Default|GetCodePiece)))

(fn SetRotation
  (params (Rotation :type Direction%20Enum :default "NewEnumerator0"))
  (Variables|Default|SetRotation Rotation)
  (Transformation|SetWorldRotation (Variables|Default|GetScene) (Math|Rotator|MakeRotator 0.0 0.0 (* (Math|Conversions|ToInteger(Byte) (Variables|Default|GetRotation)) 9e+01)) false false)
  (Transformation|SetWorldRotation (Variables|Default|GetWidget) (Math|Rotator|MakeRotator 0.0 9e+01 1.8e+02) false false))

(fn SetXYR
  (params (GridX :type Integer) (GridY :type Integer) (Rotation :type Direction%20Enum :default "NewEnumerator0"))
  (bind _codepiece (Variables|Default|GetCodePiece))
  (Variables|Default|SetGridX GridX)
  (Variables|Default|SetGridY GridY)
  (Variables|Default|SetRotation Rotation)
  (Variables|/Game/Deadbit/Blueprints/BotProgramming/Functions/BaseClasses/CodePiece.CodePiece_C|SetGridX _codepiece GridX)
  (Variables|/Game/Deadbit/Blueprints/BotProgramming/Functions/BaseClasses/CodePiece.CodePiece_C|SetGridY _codepiece GridY)
  (Variables|/Game/Deadbit/Blueprints/BotProgramming/Functions/BaseClasses/CodePiece.CodePiece_C|SetRotation _codepiece Rotation))