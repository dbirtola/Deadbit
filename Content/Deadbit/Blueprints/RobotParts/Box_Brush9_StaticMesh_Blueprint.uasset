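; Robot part Blueprint built on a static mesh that acts as a damageable shield.
; AnyDamage forwards the hit to a Health component and flashes the mesh by briefly switching the LowHealth material scalar on.
; After the flash, health at or below 30 turns LowHealth back on and leaves it on.
; Debug prints report hits and health, and nothing here handles destruction.
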(event Game|Damage|EventAnyDamage
  (params (Damage :type Float%20%28single-precision%29) (DamageType :type Damage%20Type%20Object%20Reference) (InstigatedBy :type Controller%20Object%20Reference) (DamageCauser :type Actor%20Object%20Reference))
  (bind _staticmeshcomponent (Variables|Debug|GetStaticMeshComponent))
  (bind _health (Variables|Default|GetHealth))
  (bind _health_2 (Variables|/Game/Deadbit/Blueprints/Health/Health.Health_C|GetHealth _health))
  (Development|PrintString "HIT SHIELD! DAMAGE TAKEN")
  (Default|TakeDamage _health Damage InstigatedBy DamageCauser)
  (Rendering|Material|SetScalarParameterValueonMaterials _staticmeshcomponent "LowHealth" 1.0)
  (Utilities|FlowControl|Delay 0.2)
  (Rendering|Material|SetScalarParameterValueonMaterials _staticmeshcomponent "LowHealth" 0.0)
  (Development|PrintString (Utilities|String|ToString(Float) _health_2) true true "(R=0.000000,G=0.660000,B=1.000000,A=1.000000)" _health_2)
  (Math|Float|CompareFloat _health_2 3e+01
    (:==
      _)
    (:<
      _))
  (Rendering|Material|SetScalarParameterValueonMaterials (Variables|Debug|GetStaticMeshComponent) "LowHealth" 1.0)
  (Development|PrintString (Utilities|String|ToString(Float) (Math|Conversions|ToFloat(Integer) (Utilities|GetDisplayName _health)))))

(fn ConstructionScript)