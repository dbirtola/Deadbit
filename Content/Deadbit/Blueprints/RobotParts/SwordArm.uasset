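; SwordArm is a robot part Blueprint for a sword melee attack on modular robots, currently left unwired.
; The Slash event and Slash2 function are empty at their entries.
; Disconnected logic rotates the mesh, damages the first other robot overlapping the capsule, and plays punch particles and sound.
; A timer-driven ReturnSword event resets the rotation as an animation placeholder, but its timer setup is also disconnected.
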(event Custom|ReturnSword
  ;[1 1 1] Reset the arms location. Replace this all with an animation later
  (Transformation|SetRelativeRotation (Variables|Default|GetStaticMesh) "0, 0, 0" false false))

(event Collision|EventActorBeginOverlap
  (params (OtherActor :type Actor%20Object%20Reference))
  (|CallParentFunction OtherActor) ; This node is disabled and will not be called.\nDrag off pins to build functionality.
)

(event EventTick
  (params (DeltaSeconds :type Float%20%28single-precision%29))
  (|CallParentFunction DeltaSeconds) ; This node is disabled and will not be called.\nDrag off pins to build functionality.
)

(event EventBeginPlay
  (|CallParentFunction) ; This node is disabled and will not be called.\nDrag off pins to build functionality.
)

(event EventSlash)

(fn ConstructionScript
  (|CallParentFunction))

(fn Slash2)