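; Modular hovering robot pawn that fights by faction and can be inspected when dead, revived, or edited by its owning player.
; Arms and other parts attach to body sockets through a slot map, mirroring right arms and dropping as pickups on death.
; A program from ProgramFactory runs on the Idle event, with vision-sphere and line-trace checks finding enemies.
; Tick snaps the bobbing capsule above the actor root, working around physics breaking attachment on revive.
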(event Custom|RobotDeath
  (Variables|Default|SetKilledAtLeastOnce true)
  (Variables|Default|SetFaction self "NewEnumerator2")
  (bind _keys (Utilities|Map|Keys (Variables|Default|GetEquippedParts)))
  (for _array_element _keys
    (CallFunction|DropPart _array_element))
  (Physics|SetSimulatePhysics (Variables|Default|GetCapsule) true)
  ;[1 1 1] Hide health bar of dead robots
  (Rendering|SetVisibility (Variables|Default|GetWidget) false true)
  (Audio|PlaySoundatLocation "/Game/Deadbit/Sound/SoundCues/SparkDeath.SparkDeath" (Transformation|GetActorLocation) "0, 0, 0" 1.0 1.0 0.0 0 0 0)
  (bind _asrobot_health_bar (Utilities|Casting|CastToRobotHealthBar (UserInterface|GetUserWidgetObject (Variables|Default|GetWidget)))
    (:then
      (Default|SetAlly _asrobot_health_bar false))
    (:CastFailed
      _))
  (bind _event (Default|GetEventbyName (Variables|Default|GetEventQueueComponent) "Idle"))
  (Utilities|IsValid _event
    (:Is%20Valid
      (Utilities|IsValid (Variables|/Game/Deadbit/Blueprints/BotProgramming/Events/ProgramEvent.ProgramEvent_C|GetBoundProgram _event)
        (:Is%20Valid
          (Default|Abort (Variables|/Game/Deadbit/Blueprints/BotProgramming/Events/ProgramEvent.ProgramEvent_C|GetBoundProgram _event)))))))

(event Custom|ToggleCombatState
  (bind _self self)
  (if (Utilities|Enum|Equal(Enum) (Utilities|Enum|LiteralenumFactions "NewEnumerator0") (Variables|Default|GetFaction _self))
    (bind _seenenemies (CallFunction|GetVisibleEnemies _self))
    (if (== (Utilities|Array|Length _seenenemies) 0)
      (Variables|Default|SetCircuitBreakerInCombat false)
      (else
        (Variables|Default|SetCircuitBreakerInCombat true)))
    (Default|CallCombatState)))

(event Custom|Revive
  (params (HealthPercent :type Float%20%28single-precision%29))
  (bind _cube (Variables|Default|GetCube))
  (bind _capsule (Variables|Default|GetCapsule))
  (bind _returnvalue (Transformation|GetWorldLocation _cube))
  (Variables|/Game/Deadbit/Blueprints/Health/Health.Health_C|SetHealth (Variables|Default|GetHealth) (* HealthPercent (Variables|/Game/Deadbit/Blueprints/Health/Health.Health_C|GetmaxHealth (Variables|Default|GetHealth))))
  (Physics|SetSimulatePhysics (Variables|Default|GetCapsule) false)
  (Transformation|SetWorldRotation _capsule (Math|Rotator|MakeRotator 0.0 0.0 (.yaw (Transformation|GetWorldRotation _capsule))) false false)
  ;[1 1 1] Move the capsule to the location of the body since attaching isnt working through blueprints. Remove when attachment issue is figured out.
  (Transformation|SetWorldLocation (Variables|Default|GetGroundPosition) (Transformation|GetWorldLocation (Variables|Default|GetCapsule)) false false)
  (Transformation|AttachComponentToComponent (Variables|Default|GetCapsule) (Variables|Default|GetGroundPosition) "None" "KeepRelative" "SnapToTarget" "KeepWorld" true)
  (Transformation|SetRelativeLocation (Variables|Default|GetCapsule) (Math|Vector|MakeVector 0.0 0.0 (Variables|Default|GetFlyHeight)) false false)
  (Audio|PlaySoundatLocation "/Game/Deadbit/Sound/SoundCues/RobotRecruit.RobotRecruit" _returnvalue "0, 0, 0" 1.0 1.0 0.0 0 0 0)
  (Effects|SpawnEmitteratLocation "/Game/Deadbit/Cascade/P_ZoeyTakeDamage.P_ZoeyTakeDamage" _returnvalue)
  (Default|CallRobotModified self))

(event EventBeginPlay
  (bind _spawnedrightarm (Variables|DefaultParts|GetSpawnedRightArm))
  (bind _health (Variables|Default|GetHealth))
  (bind _spawnedleftarm (Variables|DefaultParts|GetSpawnedLeftArm))
  (Utilities|FlowControl|Sequence
    (:then_0
      ;[1 1 1] Initializing components and program
      (Default|Initialize (.AsRobot%20Health%20Bar (Utilities|Casting|CastToRobotHealthBar (UserInterface|GetUserWidgetObject (Variables|Default|GetWidget)))) self))
    (:then_1
      ;[1 1 1] Spawning default parts set through the inspector or from the exposed variables in the Spawn Actor node
      (if (not (and (<= (Variables|/Game/Deadbit/Blueprints/Health/Health.Health_C|GetHealth _health) 0.0) (not (Variables|/Game/Deadbit/Blueprints/Health/Health.Health_C|GetStartWithMax _health))))
        (Utilities|FlowControl|Sequence
          (:then_0
            (if (Utilities|IsValidClass _spawnedleftarm)
              (bind _returnvalue (Game|SpawnActorfromClass _spawnedleftarm (Math|Transform|MakeTransform "0, 0, 0" "0, 0, 0" "0.900000,0.900000,0.900000") "Undefined" self 0))
              (CallFunction|EquipPart _returnvalue (Variables|/Game/Deadbit/Blueprints/RobotParts/RobotPart.RobotPart_C|GetSlot _returnvalue) true)))
          (:then_1
            ;[1 1 1] Spawning default parts set through the inspector or from the exposed variables in the Spawn Actor node
            (if (Utilities|IsValidClass _spawnedrightarm)
              (bind _returnvalue_2 (Game|SpawnActorfromClass _spawnedrightarm (Math|Transform|MakeTransform "0, 0, 0" "0, 0, 0" "0.900000,0.900000,0.900000") "Undefined" self 0))
              (CallFunction|EquipPart _returnvalue_2 "NewEnumerator2" true))))))
    (:then_2
      ;[1 1 1] Randomize initial values to gives robots some variance
      (bind _name (CallFunction|RandomizeName))
      (Variables|Default|SetRobotName _name)
      (Default|CallRobotModified self)
      (Variables|Default|SetHover%20Speed (+ (Variables|Default|GetHover%20Speed) (Math|Random|RandomFloatinRange -2.0 2.0)))
      (Variables|Default|SetHoverAmplitude (+ (Variables|Default|GetHoverAmplitude) (Math|Random|RandomFloatinRange -15.0 15.0))))
    (:then_3
      (EventDispatchers|BindEventtoDeath (Variables|Default|GetHealth) (delegate Custom|RobotDeath))
      (Utilities|FlowControl|Delay 0.2)
      (bind _outactors (Actor|GetAllActorsOfClass "/Game/Deadbit/Blueprints/BotProgramming/ProgramFactory.ProgramFactory_C"))
      (bind _program (Default|MakeProgrambyName (Utilities|Array|Get(acopy) _outactors) (Variables|Default|GetProgram%20Name)))
      (Utilities|IsValid _program
        (:Is%20Valid
          (bind _event (Default|GetEventbyName (Variables|Default|GetEventQueueComponent) "Idle"))
          (Utilities|IsValid _program
            (:Is%20Valid
              (Default|BindProgramtoEvent _event _program)
              (Default|StartProgram _program))))))))

(event EventTick
  (params (DeltaSeconds :type Float%20%28single-precision%29))
  ;[1 1 1] If the robot is alive we want to snap him to the location of the root component. There is an issue with the way UE4 handles physics that is preventing us from "reconnecting" the capsule component to the root component when a robot is revived.
  ; TODO: Try moving this to C++ for a bit more control over the hierarchy
  (bind _alive (Default|IsAlive (Variables|Default|GetHealth)))
  (Variables|Default|SetHoverOffset (* (Math|Trig|Sin(Degrees) (* (Actor|GetGameTimeSinceCreation) (Variables|Default|GetHover%20Speed))) (Variables|Default|GetHoverAmplitude)))
  (if _alive
    (Transformation|SetWorldLocation (Variables|Default|GetCapsule) (+ (Transformation|GetActorLocation) (Math|Vector|MakeVector 0.0 0.0 (+ (Variables|Default|GetFlyHeight) (Variables|Default|GetHoverOffset)))) false false)))

(event EventMove
  (params (Target :type Vector :default "0, 0, 0") (TargetACtor :type Actor%20Object%20Reference))
  (bind _returnvalue (Transformation|GetActorLocation))
  (bind _returnvalue_2 (- Target _returnvalue))
  (bind _returnvalue_3 (Math|Vector|VectorLength _returnvalue_2))
  (bind _returnvalue_4 (Class|NavigationSystemV1|FindPathtoLocationSynchronously (AI|GetAIController self) (Transformation|GetActorLocation) Target self 0))
  (if (< _returnvalue_3 (Variables|Default|GetStepSize))
    (AI|AIMoveTo self (+ (Transformation|GetActorLocation) (* (Math|Vector|Normalize _returnvalue_2) (- _returnvalue_3 1e+02))) 0 2e+01 false)
    (else
      (AI|AIMoveTo self (+ (Transformation|GetActorLocation) (* (Math|Vector|Normalize (- (Utilities|Array|Get(acopy) (Variables|/Script/NavigationSystem.NavigationPath|GetPathPoints _returnvalue_4) 1) (Transformation|GetActorLocation))) (Variables|Default|GetStepSize))) 0 1e+01 false))))

(fn ConstructionScript
  (Transformation|SetRelativeLocation (Variables|Default|GetCapsule) (Math|Vector|MakeVector 0.0 0.0 (Variables|Default|GetFlyHeight)) false false))

(fn GetAvailableCodePieces
  (return (Variables|Default|GetDefault%20Pieces)))

(fn EquipPart
  (params (Part :type Robot%20Part%20Object%20Reference) (Slot :type RobotPartSlots%20Enum :default "NewEnumerator5") (Snap%20to%20ground? :type Boolean))
  (bind _returnvalue (Components|GetOwner))
  (bind _equippedparts (Variables|Default|GetEquippedParts))
  (bind _output_get (LocalVariables|SetTarget%20Part Part))
  (LocalVariables|SetTarget%20Slot (Variables|/Game/Deadbit/Blueprints/RobotParts/RobotPart.RobotPart_C|GetSlot _output_get))
  (if (or (Utilities|Enum|Equal(Enum) (Variables|/Game/Deadbit/Blueprints/RobotParts/RobotPart.RobotPart_C|GetSlot _output_get) "NewEnumerator1") (Utilities|Enum|Equal(Enum) (Variables|/Game/Deadbit/Blueprints/RobotParts/RobotPart.RobotPart_C|GetSlot _output_get) "NewEnumerator2"))
    (bind _output_get_2 (LocalVariables|SetTarget%20Slot Slot)))
  (LocalVariables|SetSnap%20to%20ground Snap%20to%20ground?)
  (if (Math|Boolean|ANDBoolean (Utilities|Enum|Equal(Enum) _output_get_2 "NewEnumerator1") (.ReturnValue (Utilities|Map|Find _equippedparts "NewEnumerator1")) (not (.ReturnValue (Utilities|Map|Find _equippedparts "NewEnumerator2"))))
    (LocalVariables|SetTarget%20Slot "NewEnumerator2"))
  (Utilities|FlowControl|Sequence
    (:then_0
      (CallFunction|UnequipPart (LocalVariables|GetTarget%20Slot))
      (Utilities|IsValid _returnvalue
        (:Is%20Valid
          (bind _ascbplayer_controller (Utilities|Casting|CastToCBPlayerController (Game|GetInstigatorController _returnvalue)))
          (Default|RemovePart _ascbplayer_controller (LocalVariables|GetTarget%20Part)))))
    (:then_1
      (Utilities|Map|Add (Variables|Default|GetEquippedParts) (LocalVariables|GetTarget%20Slot) (LocalVariables|GetTarget%20Part))
      ;[1 1 1] Determine which socket we need to attach to
      (switch Utilities|FlowControl|Switch|SwitchonRobotPartSlots (LocalVariables|GetTarget%20Slot)
        (:NewEnumerator0
          (LocalVariables|SetSocketName "Head"))
        (:NewEnumerator1
          (LocalVariables|SetSocketName "LeftArm"))
        (:NewEnumerator2
          (LocalVariables|SetSocketName "RightArm")
          (Transformation|SetActorScale3D (LocalVariables|GetTarget%20Part) (* (Variables|/Game/Deadbit/Blueprints/RobotParts/RobotPart.RobotPart_C|GetDesiredScale (LocalVariables|GetTarget%20Part)) "1.000000,-1.000000,1.000000")))
        (:NewEnumerator3
          (LocalVariables|SetSocketName "Legs"))
        (:NewEnumerator4
          (LocalVariables|SetSocketName "Back"))))
    (:then_2
      ;[1 1 1] Actual equipping of part
      (Transformation|AttachComponentToComponent (LocalVariables|GetTarget%20Part) (Variables|Default|GetCube) (LocalVariables|GetSocketName) "SnapToTarget" "SnapToTarget" "KeepRelative" true)
      (bind _output_get_3 (Variables|/Game/Deadbit/Blueprints/RobotParts/RobotPart.RobotPart_C|SetOwningRobot (LocalVariables|GetTarget%20Part) self))
      ;[1 1 1] Make part visible and snap the robot to the ground (since height can change)
      (Default|EquiptoRobot (LocalVariables|GetTarget%20Part) _output_get_3)
      (Rendering|SetVisibility (Variables|/Script/Engine.Actor|GetRootComponent (LocalVariables|GetTarget%20Part)) true true)
      (Audio|PlaySound2D "/Game/Deadbit/Sound/SoundCues/Equip.Equip" 1.0 1.0 0.0 0 0)
      (Default|CallRobotModified self (LocalVariables|GetTarget%20Part)))))

(fn UnequipPart
  (params (Slot :type RobotPartSlots%20Enum :default "NewEnumerator5"))
  (bind _returnvalue (Components|GetOwner))
  (bind _equippedparts (Variables|Default|GetEquippedParts))
  (bind (_value _returnvalue_2) (Utilities|Map|Find _equippedparts Slot))
  (if _returnvalue_2
    (bind _output_get (LocalVariables|SetPart _value))
    (Transformation|DetachFromActor _value "KeepRelative" "KeepRelative" "KeepRelative")
    ;[1 1 1] In case it was a right arm and had its scale flipped
    (Transformation|SetActorScale3D (LocalVariables|GetPart) "1.000000,1.000000,1.000000")
    (Utilities|IsValid _returnvalue
      (:Is%20Valid
        (bind _ascbplayer_controller (Utilities|Casting|CastToCBPlayerController (Game|GetInstigatorController _returnvalue)))
        (Utilities|Array|Add (Variables|/Game/Deadbit/Blueprints/CBPlayerController.CBPlayerController_C|GetOwnedParts _ascbplayer_controller) (LocalVariables|GetPart))))))

(fn SnaptoGround)

(fn GetVisibleEnemies
  (bind _output_get (LocalVariables|SetOverlappingActors (Collision|GetOverlappingActors (Variables|Default|GetVisionSphere) "ModularRobot_C" :!class /Script/Engine.PrimitiveComponent)))
  (Utilities|Array|RemoveItem _output_get self)
  (Utilities|Array|AppendArray _output_get (Collision|GetOverlappingActors (Variables|Default|GetVisionSphere) "/Game/Deadbit/Blueprints/ThirdPersonCharacter/PlayerCharacter.PlayerCharacter_C" :!class /Script/Engine.PrimitiveComponent))
  (for _array_element _output_get
    (bind _asmodular_robot (Utilities|Casting|CastToModularRobot _array_element)
      (:then
        ;[1 1 1] Remove invalid modular robots
        (if (and (Utilities|Enum|NotEqual(Enum) (Variables|ModularRobot_C|GetFaction _asmodular_robot) (Variables|Default|GetFaction)) (> (Variables|/Game/Deadbit/Blueprints/Health/Health.Health_C|Gethealth (Variables|ModularRobot_C|GetHealth _asmodular_robot)) 0.0))
          (bind _returnvalue (Collision|LineTraceForObjects (Transformation|GetWorldLocation (Variables|ModularRobot_C|GetCube _asmodular_robot)) (Transformation|GetWorldLocation (Variables|Default|GetCube)) (Utilities|Array|MakeArray "ObjectTypeQuery1") false (Utilities|Array|MakeArray (Game|Player|GetPlayerPawn 0)) "None"))
          (if (not _returnvalue)
            (Utilities|Array|Add (LocalVariables|GetVisibleEnemies) _asmodular_robot))))
      (:CastFailed
        (if (Utilities|Enum|NotEqual(Enum) (Variables|Default|GetFaction) "NewEnumerator0")
          (bind _asplayer_character (Utilities|Casting|CastToPlayerCharacter _array_element))
          (if (> (Variables|/Game/Deadbit/Blueprints/Health/Health.Health_C|GetHealth (Variables|/Game/Deadbit/Blueprints/ThirdPersonCharacter/PlayerCharacter.PlayerCharacter_C|GetHealth _asplayer_character)) 0.0)
            (bind _returnvalue_2 (Collision|LineTraceForObjects (Transformation|GetWorldLocation (Variables|Default|GetCube)) (Transformation|GetWorldLocation (Variables|/Script/Engine.Character|GetMesh _asplayer_character)) (Utilities|Array|MakeArray "ObjectTypeQuery1") false (Utilities|Array|MakeArray 0) "None"))
            (if (not _returnvalue_2)
              (Utilities|Array|Add (LocalVariables|GetVisibleEnemies) _asplayer_character)))))))
  (if (> (Utilities|Array|Length (LocalVariables|GetVisibleEnemies)) 0)
    (Variables|Default|SetCircuitBreakerInCombat true)
    (if (Utilities|IsValid (Variables|Default|GetSpawnedHostileParticle))
      _
      (else
        (bind _returnvalue_3 (Effects|SpawnEmitterAttached "/Game/Deadbit/Cascade/P_EnemyLigtht.P_EnemyLigtht" (Variables|Default|GetCube) "None" "30.000000, 0, 0" "0, 0, 0" "1.000000,1.000000,1.000000" "SnapToTarget" false))
        (Variables|Default|SetSpawnedHostileParticle _returnvalue_3)))
    (else
      (Variables|Default|SetCircuitBreakerInCombat false)))
  (Default|CallCombatState)
  (return (LocalVariables|GetVisibleEnemies)))

(fn AssignOwnership
  (params (Owning%20Character :type Actor%20Object%20Reference))
  (bind _capsule (Variables|Default|GetCapsule))
  (Actor|SetOwner Owning%20Character)
  (Variables|Default|SetFaction "NewEnumerator0")
  (Collision|SetCollisionResponsetoChannel _capsule "ECC_GameTraceChannel1" "ECR_Ignore")
  (Collision|SetCollisionResponsetoChannel _capsule "ECC_GameTraceChannel2" "ECR_Block")
  (return))

(fn RandomizeName
  (bind _array (Utilities|Array|MakeArray "John" "Tristan" "Luke" "Damen" "Alexai" "Matt" "Milo" "Zack" "David" "Abdul"))
  (return (Utilities|String|Append (Utilities|Array|Get(acopy) _array (Math|Random|RandomInteger (Utilities|Array|Length _array))) "Bot")))

(fn ChangeName
  (params (New%20Name :type String))
  (Variables|Default|SetRobotName New%20Name)
  (Default|CallRobotModified self))

(fn DropPart
  (params (PartSlot :type RobotPartSlots%20Enum :default "NewEnumerator5"))
  (bind _equippedparts (Variables|Default|GetEquippedParts))
  (bind (_value _returnvalue) (Utilities|Map|Find _equippedparts PartSlot))
  (if _returnvalue
    (LocalVariables|SetPart _value)
    (Transformation|DetachFromActor (LocalVariables|GetPart) "KeepWorld" "KeepRelative" "KeepRelative")
    ;[1 1 1] In case it was a right arm and had its scale flipped
    (Transformation|SetActorScale3D (LocalVariables|GetPart) "1.000000,1.000000,1.000000")
    (Default|Unequip (LocalVariables|GetPart))
    (Default|SetPickupable (LocalVariables|GetPart) true)
    (Collision|SetCollisionEnabled (Variables|/Game/Deadbit/Blueprints/RobotParts/RobotPart.RobotPart_C|GetRobotPart (LocalVariables|GetPart)) "QueryAndPhysics")
    (Utilities|Map|Remove (Variables|Default|GetEquippedParts) PartSlot)
    (return (LocalVariables|GetPart))))

(fn GetInfo
  (params (Interactor :type Controller%20Object%20Reference))
  (if (<= (Variables|/Game/Deadbit/Blueprints/Health/Health.Health_C|Gethealth (Variables|Default|GetHealth)) 0.0)
    (return true "Inspect")
    (elif (== (Pawn|GetControlledPawn (Game|GetPlayerController 0)) (Components|GetOwner))
      (return true "Edit")
      (else
        (return false "Hack")))))

(fn Interact
  (params (Interactor :type CB%20Player%20Controller%20Object%20Reference))
  (bind _self self)
  (Development|PrintString (Utilities|String|ToString(Integer) (Utilities|Array|Length (Variables|/Game/Deadbit/Blueprints/BotProgramming/EventQueueComponent.EventQueueComponent_C|GetQueuedEvents (Variables|Default|GetEventQueueComponent)))))
  (if (<= (Variables|/Game/Deadbit/Blueprints/Health/Health.Health_C|Gethealth (Variables|Default|GetHealth)) 0.0)
    (Default|InspectRobot Interactor _self)
    (Development|PrintString (Utilities|String|ToString(Integer) (Utilities|Array|Length (Variables|/Game/Deadbit/Blueprints/BotProgramming/EventQueueComponent.EventQueueComponent_C|GetQueuedEvents (Variables|Default|GetEventQueueComponent)))))
    (elif (== (Pawn|GetControlledPawn (Game|GetPlayerController 0)) (Components|GetOwner))
      (Default|EditRobot Interactor _self))))