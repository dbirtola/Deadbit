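; BasicArm is a robot arm part for modular robots that exposes a Punch action.
; Punch ignores calls while Punching is set; otherwise Punch2 sets that flag and a half-second timer clears it through ReturnArm.
; The arm rotation and the damage, particle and sound hit on an overlapping ModularRobot are disconnected, so a punch currently only toggles the flag.
; A note marks the rotation reset for replacement by animation.
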(event Custom|ReturnArm
  ;[1 1 1] Reset the arms location. Replace this all with an animation later
  (Variables|Default|SetPunching false))

(event EventPunch
  (if (not (Variables|Default|GetPunching))
    ;[1 1 1] Reset the arms location. Replace this all with an animation later
    (CallFunction|Punch2)
    (Utilities|Time|SetTimerbyEvent (delegate Custom|ReturnArm) 0.5)))

(fn ConstructionScript
  (|CallParentFunction))

(fn Punch2
  (Variables|Default|SetPunching true))