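; RobotPart is a base pickup actor for robot body parts that can be collected, equipped to a robot and dropped.
; Interacting with a pickupable part hides it, disables its physics and collision, and hands it to the interactor; equipping shows it again, while unequipping re-enables physics and pickup.
; A dynamic material's glow parameter marks pickupable parts, and damage taken is forwarded to the attach parent actor.
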(event Custom|EquipToRobot
  (params (Robot :type Modular%20Robot%20Object%20Reference))
  (bind _dynamicmaterialreference (Variables|Default|GetDynamicMaterialReference))
  (Variables|Default|SetOwningRobot Robot)
  (Utilities|IsValid _dynamicmaterialreference
    (:Is%20Valid
      (Rendering|Material|SetScalarParameterValue _dynamicmaterialreference "ShouldGlow" 0.0 :!class /Script/Engine.MaterialInstanceDynamic)
      (Rendering|SetVisibility (Variables|Default|GetRobotPart) true true)
      (Collision|SetCollisionEnabled (Variables|Default|GetRobotPart) "QueryAndPhysics"))))

(event Custom|SetPickupable
  (params (Pickupable :type Boolean))
  (bind _output_get (Variables|Default|SetPickUpable Pickupable))
  (if _output_get
    (Rendering|Material|SetScalarParameterValue (Variables|Default|GetDynamicMaterialReference) "ShouldGlow" 1.0 :!class /Script/Engine.MaterialInstanceDynamic)))

(event Game|Damage|EventAnyDamage
  (params (Damage :type Float%20%28single-precision%29) (DamageType :type Damage%20Type%20Object%20Reference) (InstigatedBy :type Controller%20Object%20Reference) (DamageCauser :type Actor%20Object%20Reference))
  (Game|Damage|ApplyDamage (Actor|GetAttachParentActor) Damage InstigatedBy DamageCauser))

(fn ConstructionScript
  (Transformation|SetRelativeScale3D (Variables|Default|GetRobotPart) (Variables|Default|GetDesiredScale))
  (bind _returnvalue (Rendering|Material|CreateDynamicMaterialInstance (Variables|Default|GetRobotPart) 0 (Variables|Default|GetMaterialLayer) "None" :!class /Script/Engine.PrimitiveComponent))
  (Variables|Default|SetDynamicMaterialReference _returnvalue)
  (if (Variables|Default|GetPickUpable)
    (Rendering|Material|SetScalarParameterValue (Variables|Default|GetDynamicMaterialReference) "ShouldGlow" 1.0 :!class /Script/Engine.MaterialInstanceDynamic)))

(fn PickUp
  (if (Variables|Default|GetPickUpable)
    (CallFunction|SetPickupable false)
    (Rendering|SetVisibility (Variables|Transformation|GetRootComponent) false true)
    (Physics|SetSimulatePhysics (Variables|Default|GetRobotPart) false)
    (Collision|SetCollisionEnabled (Variables|Default|GetRobotPart) "NoCollision")
    (return true)))

(fn Unequip
  (bind _returnvalue (Actor|GetParentActor))
  (Variables|Default|SetOwningRobot 0)
  (Physics|SetSimulatePhysics (Variables|Default|GetRobotPart) true)
  (CallFunction|SetPickupable true)
  ;[1 1 1] If this part is attached to something, detach it
  (if (Utilities|IsValid _returnvalue)
    (Transformation|DetachFromActor _returnvalue "KeepRelative" "KeepRelative" "KeepRelative"))
  ;[1 1 1] In case it was a right arm and had its scale flipped
  (Transformation|SetActorScale3D self (Variables|Default|GetDesiredScale)))

(fn GetInfo
  (params (Interactor :type Controller%20Object%20Reference))
  (if (Variables|Default|GetPickUpable)
    (return (Variables|Default|GetPickUpable) (Utilities|String|Append "Pick up " (Variables|Default|GetPart%20Name)))
    (else
      (return (Variables|Default|GetPickUpable) ""))))

(fn Interact
  (params (Interactor :type CB%20Player%20Controller%20Object%20Reference))
  (if (Variables|Default|GetPickUpable)
    (bind _success (CallFunction|PickUp))
    (if true
      (Default|PickupPart Interactor self))
    (return _success)
    (else
      (return false))))