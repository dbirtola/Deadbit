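; BasicLegs is a robot part Blueprint that provides movement for the robot that owns it.
; Its Move event issues an AI MoveTo on the owning robot toward the given target, with a fixed acceptance radius and no handling of success or failure.
; The default BeginPlay, overlap and Tick events are disabled, and the construction script only calls its parent.
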(event EventBeginPlay
  (|CallParentFunction) ; This node is disabled and will not be called.\nDrag off pins to build functionality.
)

(event Collision|EventActorBeginOverlap
  (params (OtherActor :type Actor%20Object%20Reference))
  (|CallParentFunction OtherActor) ; This node is disabled and will not be called.\nDrag off pins to build functionality.
)

(event EventTick
  (params (DeltaSeconds :type Float%20%28single-precision%29))
  (|CallParentFunction DeltaSeconds) ; This node is disabled and will not be called.\nDrag off pins to build functionality.
)

(event EventMove
  (params (Target :type Vector :default "0, 0, 0"))
  (bind _owningrobot (Variables|Default|GetOwningRobot))
  (AI|AIMoveTo (AI|GetAIController _owningrobot) _owningrobot Target 0 1.5e+02 false))

(fn ConstructionScript
  (|CallParentFunction))