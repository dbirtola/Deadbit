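; ShieldBest is a damageable robot-part shield that is owned by a ShieldArm.
; It forwards any damage to its Health component with debug prints, and destroys itself when that component signals death.
; On BeginPlay it reads the owning ShieldArm's faction to set its collision box to block one of two custom trace channels and ignore the other.
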(event Custom|ShieldKIll
  (Actor|DestroyActor self))

(event EventBeginPlay
  (bind _collision_box (Variables|Default|Getcollision%20box))
  (bind _collision_box_2 (Variables|Default|Getcollision%20box))
  (|CallParentFunction)
  (EventDispatchers|BindEventtoDeath (Variables|Default|GetHealth) (delegate Custom|ShieldKIll))
  (|CallParentFunction)
  (bind _asshield_arm (Utilities|Casting|CastToShieldArm (Components|GetOwner self)))
  (if (== (Variables|/Game/Deadbit/Blueprints/RobotParts/ShieldArm.ShieldArm_C|GetFaction _asshield_arm) (Utilities|Enum|LiteralenumFactions "NewEnumerator0"))
    (Collision|SetCollisionResponsetoChannel _collision_box_2 "ECC_GameTraceChannel1" "ECR_Ignore")
    (Collision|SetCollisionResponsetoChannel _collision_box_2 "ECC_GameTraceChannel2" "ECR_Block")
    (else
      (Collision|SetCollisionResponsetoChannel _collision_box "ECC_GameTraceChannel1" "ECR_Block")
      (Collision|SetCollisionResponsetoChannel _collision_box "ECC_GameTraceChannel2" "ECR_Ignore"))))

(event Game|Damage|EventAnyDamage
  (params (Damage :type Float%20%28single-precision%29) (DamageType :type Damage%20Type%20Object%20Reference) (InstigatedBy :type Controller%20Object%20Reference) (DamageCauser :type Actor%20Object%20Reference))
  (bind _health (Variables|Default|GetHealth))
  (Development|PrintString "HIT SHIELD! DAMAGE TAKEN")
  (Default|TakeDamage _health Damage InstigatedBy DamageCauser)
  (Development|PrintString (Utilities|String|ToString(Float) (Math|Conversions|ToFloat(Integer) (Utilities|GetDisplayName _health)))))

(fn ConstructionScript)