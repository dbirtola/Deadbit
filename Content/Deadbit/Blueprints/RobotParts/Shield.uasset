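; Shield is a robot part actor that takes damage and destroys itself when its health runs out.
; On begin play it binds the Health component's death event to a handler that destroys the actor.
; Any damage received is forwarded to Health, with the instigator passed as the damaged party and the causer as the damager, alongside debug prints.
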(event Custom|ShieldKIll
  (Actor|DestroyActor self))

(event Game|Damage|EventAnyDamage
  (params (Damage :type Float%20%28single-precision%29) (DamageType :type Damage%20Type%20Object%20Reference) (InstigatedBy :type Controller%20Object%20Reference) (DamageCauser :type Actor%20Object%20Reference))
  (bind _health (Variables|Default|GetHealth))
  (Development|PrintString "HIT SHIELD! DAMAGE TAKEN")
  (Default|TakeDamage _health Damage InstigatedBy DamageCauser)
  (Development|PrintString (Utilities|String|ToString(Float) (Math|Conversions|ToFloat(Integer) (Utilities|GetDisplayName _health)))))

(event Collision|EventActorBeginOverlap
  (params (OtherActor :type Actor%20Object%20Reference)))

(event EventTick
  (params (DeltaSeconds :type Float%20%28single-precision%29)))

(event EventBeginPlay
  (|CallParentFunction)
  (EventDispatchers|BindEventtoDeath (Variables|Default|GetHealth) (delegate Custom|ShieldKIll)))

(fn ConstructionScript)