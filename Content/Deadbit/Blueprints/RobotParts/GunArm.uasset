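; GunArm is a robot part Blueprint that fires bullets at a target location on behalf of its owning robot.
; Shoot rotates the arm mesh, spawns a scaled-down Bullet at BulletSpawn with the robot as instigator, and aims its projectile velocity at the target.
; It also plays a gunshot emitter at the muzzle, then a short timer calls ReturnHand to reset the arm's rotation.
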(event Custom|ReturnHand
  (Transformation|SetRelativeRotation (Variables|Default|GetStaticMesh) "0, 0, 0" false false))

(event EventShoot
  (params (Target :type Vector :default "0, 0, 0"))
  (bind _bulletspawn (Variables|Default|GetBulletSpawn))
  (bind _bulletspawn_2 (Variables|Default|GetBulletSpawn))
  (bind _returnvalue (Transformation|GetWorldTransform _bulletspawn))
  (bind _returnvalue_2 (Transformation|GetWorldTransform _bulletspawn_2))
  (Transformation|SetRelativeRotation (Variables|Default|GetStaticMesh) "70.000000, 0, 0" false false)
  (bind _returnvalue_3 (Game|SpawnActorfromClass "/Game/Deadbit/Blueprints/Bullet.Bullet_C" (Math|Transform|MakeTransform (.location _returnvalue) (.rotation _returnvalue) "0.100000,0.100000,0.100000") "Undefined" self (Variables|Default|GetOwningRobot)))
  (Variables|/Script/Engine.MovementComponent|SetVelocity (Variables|/Game/Deadbit/Blueprints/Bullet.Bullet_C|GetProjectileMovement _returnvalue_3) (* (Math|Vector|Normalize (- Target (.location _returnvalue))) 2.5e+03))
  (Effects|SpawnEmitteratLocation "/Game/Deadbit/Cascade/P_GunShot.P_GunShot" (.location _returnvalue_2) (.rotation _returnvalue_2))
  (Utilities|Time|SetTimerbyEvent (delegate Custom|ReturnHand) 0.5))

(fn ConstructionScript
  (|CallParentFunction))