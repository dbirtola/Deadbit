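; ShieldArm is a robot-part Blueprint that spawns a shield when the V key is pressed.
; Each press spawns a new actor and attaches it to the Scene component, snapping location and rotation while keeping world scale, with no removal or duplicate check.
; The Block event is an empty stub, and a leftover cast to Shield is never executed.
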(event EventBeginPlay
  (|CallParentFunction) ; This node is disabled and will not be called.\nDrag off pins to build functionality.
)

(event Collision|EventActorBeginOverlap
  (params (OtherActor :type Actor%20Object%20Reference))
  (|CallParentFunction OtherActor) ; This node is disabled and will not be called.\nDrag off pins to build functionality.
)

(event EventTick
  (params (DeltaSeconds :type Float%20%28single-precision%29))
  (|CallParentFunction DeltaSeconds) ; This node is disabled and will not be called.\nDrag off pins to build functionality.
)

(event EventBlock)

(event Input|KeyboardEvents|V
  (params (Key :type Key%20Structure))
  (:Pressed
    (bind _returnvalue (Game|SpawnActorfromClass "/Game/Deadbit/Blueprints/RobotParts/Shield.Shield_C" (Math|Transform|MakeTransform "0, 0, 0" "0, 0, 0" "1,1,1") "Undefined" 0 0))
    (Transformation|AttachComponentToComponent _returnvalue (Variables|Default|GetScene) "None" "SnapToTarget" "SnapToTarget" "KeepWorld" false)))

(fn ConstructionScript
  (|CallParentFunction))