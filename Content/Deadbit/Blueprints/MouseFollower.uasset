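; MouseFollower is an actor that trails the mouse cursor on the horizontal plane at the player character's height.
; Each tick it deprojects the cursor into a long world ray and intersects it with an upward-facing plane through the character.
; It then lerps a fixed fraction from its current location toward that hit point, giving smoothed but frame-rate-dependent following without sweeping.
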(event EventBeginPlay)

(event Collision|EventActorBeginOverlap
  (params (OtherActor :type Actor%20Object%20Reference)))

(event EventTick
  (params (DeltaSeconds :type Float%20%28single-precision%29))
  (bind _returnvalue (Game|GetPlayerController 0))
  (bind (_worldlocation _worlddirection) (Game|Player|ConvertMouseLocationToWorldSpace _returnvalue))
  (Transformation|SetActorLocation (Math|Vector|Lerp(Vector) (Transformation|GetActorLocation) (.Intersection (Class|KismetMathLibrary|LinePlaneIntersection _worldlocation (+ _worldlocation (* _worlddirection 1e+05)) (Class|KismetMathLibrary|MakePlanefromPointandNormal (Transformation|GetActorLocation (Game|GetPlayerCharacter 0)) "0, 0,1.000000"))) 0.2) false false))

(fn ConstructionScript)