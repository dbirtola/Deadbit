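; PartDrop is a pickup actor that displays a robot part and grants it to the player on touch.
; InitializeWithPart, run at construction and BeginPlay, shows the part as a child actor, scaled by its largest extent to fit IconBounds, rotated, without mesh shadows or collision.
; On sphere overlap by a CBPlayerController's actor, it spawns a fresh DefaultClass instance, passes it to PickupPart and destroys itself.
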(event OnComponentBeginOverlap(Sphere)
  (params (OverlappedComponent :type Primitive%20Component%20Object%20Reference) (OtherActor :type Actor%20Object%20Reference) (OtherComp :type Primitive%20Component%20Object%20Reference) (OtherBodyIndex :type Integer) (bFromSweep :type Boolean) (SweepResult :type Hit%20Result%20Structure%20%28by%20ref%29))
  (bind _ascbplayer_controller (Utilities|Casting|CastToCBPlayerController (Game|GetInstigatorController OtherActor)))
  (bind _returnvalue (Game|SpawnActorfromClass (Variables|Default|GetDefaultClass) (Math|Transform|MakeTransform "0, 0, 0" "0, 0, 0" "1,1,1") "Undefined" 0 0))
  (Default|PickupPart _ascbplayer_controller _returnvalue)
  (Actor|DestroyActor)
  (Development|PrintString "Picked up"))

(event Custom|InitializeWithPart
  (params (Part :type Robot%20Part%20Class%20Reference))
  (bind _childactor (Variables|Default|GetChildActor))
  (bind _childactor_2 (Variables|/Script/Engine.ChildActorComponent|GetChildActor _childactor))
  (ChildActorComponent|SetChildActorClass _childactor Part)
  (Transformation|AttachComponentToComponent _childactor_2 (Variables|Default|GetIconBounds) "None" "SnapToTarget" "SnapToTarget" "KeepWorld" true)
  (bind _asrobot_part (Utilities|Casting|CastToRobotPart _childactor_2))
  (Variables|Default|SetRobotPart _asrobot_part)
  (Transformation|SetActorScale3D _asrobot_part (/ (Transformation|GetActorScale3D _asrobot_part) (/ (Math|Float|Max(Float) (Math|Float|Max(Float) (.x (.BoxExtent (Collision|GetActorBounds _asrobot_part false))) (.y (.BoxExtent (Collision|GetActorBounds _asrobot_part false)))) (.z (.BoxExtent (Collision|GetActorBounds _asrobot_part false)))) (.x (.BoxExtent (Collision|GetComponentBounds (Variables|Default|GetIconBounds)))))))
  (Transformation|SetActorRotation (Variables|Default|GetRobotPart) "60.000000, 0,0.000000")
  (for _array_element (Actor|GetComponentsByClass (Variables|Default|GetRobotPart) "/Script/Engine.StaticMeshComponent")
    (Rendering|SetCastShadow _array_element false)
    (Collision|SetCollisionEnabled _array_element "NoCollision")))

(event EventBeginPlay
  (if (!= (Variables|Default|GetDefaultClass) 0)
    (CallFunction|InitializewithPart (Variables|Default|GetDefaultClass))))

(fn ConstructionScript
  (if (!= (Variables|Default|GetDefaultClass) 0)
    (CallFunction|InitializewithPart (Variables|Default|GetDefaultClass))))