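; Factory actor that builds Program actors for programmable robots, from hardcoded templates or saved data.
; Templates spawn instruction actors, with target getters as parameters, wrapped in chip widgets on the program's coordinate-keyed grid; Destroy Actor and Move to Owner are disconnected stubs.
; On BeginPlay it parses ProgramData.txt into structs, splitting on closing-brace lines.
; MakeProgramByName spawns a Program from the matching struct and sets its grid.
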(event Collision|EventActorBeginOverlap
  (params (OtherActor :type Actor%20Object%20Reference)))

(event EventTick
  (params (DeltaSeconds :type Float%20%28single-precision%29)))

(event EventBeginPlay
  (CallFunction|LoadPrograms))

(fn ConstructionScript)

(fn CreateProgramfromTemplate
  (params (Template :type ProgramTemplates%20Enum :default "NewEnumerator3") (Owner :type Modular%20Robot%20Object%20Reference))
  (bind _returnvalue (Game|SpawnActorfromClass "/Game/Deadbit/Blueprints/BotProgramming/Program.Program_C" (Math|Transform|MakeTransform "0, 0, 0" "0, 0, 0" "1,1,1") "Undefined" Owner "First Program!" 0 0))
  (Variables|Default|SetCurrentProgram _returnvalue)
  (Variables|/Game/Deadbit/Blueprints/BotProgramming/Program.Program_C|SetOwningRobot _returnvalue Owner)
  (Variables|Default|SetOwnerRobot Owner)
  (Utilities|FlowControl|Sequence
    (:then_0
      (switch Utilities|FlowControl|Switch|SwitchonProgramTemplates Template
        (:NewEnumerator0
          (Actor|DestroyActor))
        (:NewEnumerator1
          (|ShootNearestEnemy))
        (:NewEnumerator2
          (|MoveToOwner))
        (:NewEnumerator4
          (|PunchNearestEnemy))
        (:NewEnumerator5
          (|PunchNearestEnemy_2))))
    (:then_1
      (return (Variables|Default|GetCurrentProgram)))))

(fn AddCodePiece
  (params (ParentFunction :type Array%20of%20Code%20Piece%20Object%20References) (Child%20Class :type Code%20Piece%20Class%20Reference))
  (bind _returnvalue (Game|SpawnActorfromClass Child%20Class (Math|Transform|MakeTransform "0, 0, 0" "0, 0, 0" "1,1,1") "Undefined" 0 (Variables|Default|GetCurrentProgram) 0 (Variables|Default|GetOwnerRobot)))
  (Utilities|Array|Add ParentFunction _returnvalue)
  (return _returnvalue))

(fn LoadPrograms
  (bind _strings (Class|MyBlueprintFunctionLibrary|LoadStringsfromFile "ProgramData.txt"))
  (if (> (Utilities|Array|Length _strings) 1)
    (for _array_element _strings
      (Utilities|Array|Add (LocalVariables|GetStrings%20for%20this%20Program) _array_element)
      (if (Utilities|Enum|Equal(Enum) _array_element "}")
        (bind _program_struct (CallFunction|ConstructProgramStructfromStrings (LocalVariables|GetStrings%20for%20this%20Program)))
        (Utilities|Array|Add (Variables|Default|GetProgram%20Structs) _program_struct)
        (Utilities|Array|Clear (LocalVariables|GetStrings%20for%20this%20Program))))
    (return true)
    (else
      (return false))))

(fn MakeProgrambyName
  (params (Program%20Name :type String))
  (for _array_element (Variables|Default|GetProgram%20Structs)
    (if (Utilities|Enum|Equal(Enum) (.ProgramName (Utilities|Struct|BreakProgramStruct _array_element)) Program%20Name)
      (bind (_name _structure) (CallFunction|GetProgramfromStruct _array_element))
      (bind _returnvalue (Game|SpawnActorfromClass "/Game/Deadbit/Blueprints/BotProgramming/Program.Program_C" (Math|Transform|MakeTransform "0, 0, 0" "0, 0, 0" "1,1,1") "Undefined" 0 _name 0 0))
      (Default|SetNewGrid _returnvalue _structure)
      (return _returnvalue))))