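; Component on a ModularRobot that holds a priority-ordered queue of events, each bound to a program the robot runs.
; BeginPlay spawns the default events and binds programs created from templates by the ProgramFactory.
; While active, Tick starts the program of the first active event, aborts running programs lower in the list, and falls back to the last event if none is selected.
; Single-frame events deactivate after selection, guaranteeing them one frame.
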(event Custom|Initialize
  (params (Events :type Array%20of%20Program%20Event%20Object%20References))
  (Variables|Default|SetEvents Events))

(event Custom|Abort
  (Default|Abort (Variables|/Game/Deadbit/Blueprints/BotProgramming/Events/ProgramEvent.ProgramEvent_C|GetBoundProgram (Variables|Default|GetEventSelectedThisFrame))))

(event EventBeginPlay
  (Variables|Default|SetRobot (.AsModular%20Robot (Utilities|Casting|CastToModularRobot (Components|GetOwner))))
  (for (_array_element _array_index) (Variables|Default|GetDefaultEvents)
    (bind _event (CallFunction|AddEvent _array_element _array_index))
    ;[1 1 1] If there was a program that should be spawned with the event, create that and bind it to the event
    (if (Utilities|Enum|NotEqual(Enum) (Utilities|Array|Get(acopy) (Variables|Default|GetDefaultPrograms) _array_index) "NewEnumerator3")
      (bind _outactors (Actor|GetAllActorsOfClass "/Game/Deadbit/Blueprints/BotProgramming/ProgramFactory.ProgramFactory_C"))
      (bind _program (Default|CreateProgramfromTemplate (Utilities|Array|Get(acopy) _outactors) (Utilities|Array|Get(acopy) (Variables|Default|GetDefaultPrograms) _array_index) (Variables|Default|GetRobot)))
      (Default|BindProgramtoEvent _event _program))))

(event EventTick
  (params (DeltaSeconds :type Float%20%28single-precision%29))
  (bind _events (Variables|Default|GetEvents))
  (if (Variables|Default|GetActive)
    (Variables|Default|SetEventSelectedThisFrame 0)
    (bind _array_element (Utilities|Array|ForEachLoopwithBreak (Variables|Default|GetEvents))
      (:LoopBody
        (Utilities|IsValid _array_element
          (:Is%20Valid
            ;[1 1 1] If we havent found an active event this frame, check if the current event is active and that the program is not running. If so, start the program
            (Utilities|IsValid (Variables|Default|GetEventSelectedThisFrame)
              (:Is%20Valid
                ;[1 1 1] If a higher priority event was selected, abort all lower priority events if they have running programs
                (Utilities|IsValid (Variables|/Game/Deadbit/Blueprints/BotProgramming/Events/ProgramEvent.ProgramEvent_C|GetBoundProgram _array_element)
                  (:Is%20Valid
                    (if (Variables|/Game/Deadbit/Blueprints/BotProgramming/Program.Program_C|GetProgramRunning (Variables|/Game/Deadbit/Blueprints/BotProgramming/Events/ProgramEvent.ProgramEvent_C|GetBoundProgram _array_element))
                      (Default|Abort (Variables|/Game/Deadbit/Blueprints/BotProgramming/Events/ProgramEvent.ProgramEvent_C|GetBoundProgram _array_element))))))
              (:Is%20Not%20Valid
                (if (Variables|/Game/Deadbit/Blueprints/BotProgramming/Events/ProgramEvent.ProgramEvent_C|GetEventActive _array_element)
                  (Utilities|IsValid (Variables|/Game/Deadbit/Blueprints/BotProgramming/Events/ProgramEvent.ProgramEvent_C|GetBoundProgram _array_element)
                    (:Is%20Valid
                      (if (Variables|/Game/Deadbit/Blueprints/BotProgramming/Program.Program_C|GetProgramRunning (Variables|/Game/Deadbit/Blueprints/BotProgramming/Events/ProgramEvent.ProgramEvent_C|GetBoundProgram _array_element))
                        _
                        (else
                          (Default|StartProgram (Variables|/Game/Deadbit/Blueprints/BotProgramming/Events/ProgramEvent.ProgramEvent_C|GetBoundProgram _array_element))))
                      (Variables|Default|SetEventSelectedThisFrame _array_element)))))))))
      (:Completed
        (Utilities|FlowControl|Sequence
          (:then_0
            ;[1 1 1] Default to lowest priority (usually Idle) if no event was selected
            (Utilities|IsValid (Variables|Default|GetEventSelectedThisFrame)
              (:Is%20Not%20Valid
                (Variables|Default|SetEventSelectedThisFrame (Utilities|Array|Get(acopy) _events (Utilities|Array|LastIndex _events))))))
          (:then_1
            ;[1 1 1] Deactivate single frame events. Doing this here instead of inside the events ensures they will have at least one frame to run
            (for _array_element_2 (Variables|Default|GetEvents)
              (Utilities|IsValid _array_element_2
                (:Is%20Valid
                  (if (Variables|/Game/Deadbit/Blueprints/BotProgramming/Events/ProgramEvent.ProgramEvent_C|GetSingleFrame _array_element_2)
                    (Default|Deactivate _array_element_2)))))))))))

(fn Disable
  (Variables|Default|SetActive false)
  (Default|Abort (Variables|/Game/Deadbit/Blueprints/BotProgramming/Events/ProgramEvent.ProgramEvent_C|GetBoundProgram (Variables|Default|GetEventSelectedThisFrame))))

(fn AddEvent
  (params (Event%20Type :type Program%20Event%20Class%20Reference) (Index :type Integer))
  (bind _robot (Variables|Default|GetRobot))
  (bind _robot_2 (Variables|Default|GetRobot))
  (if (Utilities|IsValidClass Event%20Type)
    (bind _returnvalue (Game|SpawnActorfromClass Event%20Type (Math|Transform|MakeTransform "0, 0, 0" "0, 0, 0" "1,1,1") "AlwaysSpawn" _robot _robot 0))
    (bind _returnvalue_2 (Game|SpawnActorfromClass "/Game/Deadbit/Blueprints/BotProgramming/Program.Program_C" (Math|Transform|MakeTransform "0, 0, 0" "0, 0, 0" "1,1,1") "Undefined" 0 0))
    (Default|BindProgramtoEvent _returnvalue _returnvalue_2)
    (bind _output_get (LocalVariables|SetNewEvent _returnvalue))
    (Variables|/Game/Deadbit/Blueprints/BotProgramming/Events/ProgramEvent.ProgramEvent_C|SetOwningRobot _output_get _robot_2)
    (Actor|SetOwner _output_get _robot_2)
    (if (!= Index -1)
      (Utilities|Array|Insert (Variables|Default|GetEvents) (LocalVariables|GetNewEvent) Index)
      (else
        (Utilities|Array|Add (Variables|Default|GetEvents) (LocalVariables|GetNewEvent))))
    (return (LocalVariables|GetNewEvent))))

(fn GetEventbyName
  (params (Name :type String))
  (bind _array_element (Utilities|Array|ForEachLoopwithBreak (Variables|Default|GetEvents))
    (:LoopBody
      (if (Utilities|Enum|Equal(Enum) (Variables|/Game/Deadbit/Blueprints/BotProgramming/Events/ProgramEvent.ProgramEvent_C|GetEventName _array_element) Name)
        (return _array_element)))))