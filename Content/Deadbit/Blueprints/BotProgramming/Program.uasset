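; Bot program for the programming system, storing chip widgets in a map keyed by grid position and executing their code pieces.
; StartProgram runs the piece at FirstKey, and each finish callback steps one cell in that piece's Direction.
; An empty next cell ends the run normally, while a failed piece or empty start reports an error.
; Also supports aborting and searching pieces and parameters by class; AddCodePieceByClass is an empty stub.
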(event Custom|StartProgram
  (bind _programstructure (Variables|Default|GetProgramStructure))
  (bind _firstkey (Variables|Default|GetfirstKey))
  (bind (_value _returnvalue) (Utilities|Map|Find _programstructure _firstkey))
  (Variables|Default|SetProgramRunning true)
  (Variables|Default|SetcurrentKey _firstkey)
  (if _returnvalue
    (bind _output_get (Variables|Default|SetCurrentCodePiece (Variables|/Game/Deadbit/Blueprints/UI/ProgrammingUI/ChipWidgetOld.ChipWidgetOld_C|GetCodePiece _value)))
    (bind _asvoid_piece (Utilities|Casting|CastToVoidPiece _output_get)
      (:then
        ;[1 1 1] If the current instruction node is valid, keep executing
        (EventDispatchers|BindEventtoFinishExecuting _asvoid_piece (delegate Custom|ExecuteNextStep))
        (Default|TryExecute _asvoid_piece self))
      (:CastFailed
        (Variables|Default|SetProgramRunning false)))
    (else
      ;[1 1 1] If there is no code piece in the starting position, we will end with an error
      (Variables|Default|SetProgramRunning false)
      (Default|CallProgramFinished "NewEnumerator1"))))

(event Custom|AddNode
  (params (Key :type Int%20Point%20Structure) (ChipWidget :type Chip%20Widget%20Old%20Object%20Reference))
  (Utilities|Map|Add (Variables|Default|GetProgramStructure) Key ChipWidget))

(event Custom|ExecuteNextStep
  (params (Status :type ProgramEndStatus%20Enum :default "NewEnumerator0"))
  (if (Utilities|Enum|Equal(Enum) Status "NewEnumerator0")
    ;[1 1 1] Currently pulling the next instruction directly from the right. Once programming revamp is complete, this should get the next code piece from the one that just finished executing
    (bind _output_get (Variables|Default|SetcurrentKey (CallFunction|GetNext (Variables|/Game/Deadbit/Blueprints/BotProgramming/Functions/BaseClasses/CodePiece.CodePiece_C|GetDirection (Variables|Default|GetCurrentCodePiece)) (Variables|Default|GetcurrentKey))))
    (if (.ReturnValue (Utilities|Map|Find (Variables|Default|GetProgramStructure) _output_get))
      (bind _output_get_2 (Variables|Default|SetCurrentCodePiece (Variables|/Game/Deadbit/Blueprints/UI/ProgrammingUI/ChipWidgetOld.ChipWidgetOld_C|GetCodePiece (.Value (Utilities|Map|Find (Variables|Default|GetProgramStructure) _output_get)))))
      (Utilities|IsValid _output_get_2
        (:Is%20Valid
          (bind _asvoid_piece (Utilities|Casting|CastToVoidPiece (stale Custom|StartProgram _output_get))
            (:then
              ;[1 1 1] If the current instruction node is valid, keep executing
              (EventDispatchers|BindEventtoFinishExecuting _asvoid_piece (delegate Custom|ExecuteNextStep))
              (Default|TryExecute _asvoid_piece self))
            (:CastFailed
              (Variables|Default|SetProgramRunning false))))
        (:Is%20Not%20Valid
          ;[1 1 1] If a chip fails, then our program fails and stops executing.
          (Variables|Default|SetProgramRunning false :!label _label)
          (Default|CallProgramFinished "NewEnumerator1")))
      (else
        (Variables|Default|SetProgramRunning false)
        (Default|CallProgramFinished "NewEnumerator0")))
    (else
      (goto _label))))

(event Custom|MoveNode
  (params (OldKey :type Int%20Point%20Structure) (NewKey :type Int%20Point%20Structure) (ChipWidget :type Chip%20Widget%20Old%20Object%20Reference))
  (Utilities|Map|Remove (Variables|Default|GetProgramStructure) OldKey)
  (Utilities|Map|Add (Variables|Default|GetProgramStructure) NewKey ChipWidget))

(event Custom|RemoveNode
  (params (Key :type Int%20Point%20Structure))
  (Utilities|Map|Remove (Variables|Default|GetProgramStructure) Key))

(fn ConstructionScript)

(fn AddInstruction
  (params (Code%20Piece :type Code%20Piece%20Object%20Reference) (PreviousInstruction :type Code%20Piece%20Object%20Reference) (Direction%20from%20previous :type Direction%20Enum :default "NewEnumerator0"))
  (LocalVariables|SetPiece Code%20Piece)
  (LocalVariables|SetPrevious PreviousInstruction)
  (Utilities|FlowControl|Sequence
    (:then_0
      (switch Utilities|FlowControl|Switch|SwitchonDirection Direction%20from%20previous
        (:NewEnumerator0
          (LocalVariables|SetOffset "(X=0.000000,Y=1.000000)"))
        (:NewEnumerator3
          (LocalVariables|SetOffset "(X=1.000000,Y=0.000000)"))
        (:NewEnumerator1
          (LocalVariables|SetOffset "(X=0.000000,Y=-1.000000)"))
        (:NewEnumerator2
          (LocalVariables|SetOffset "(X=-1.000000,Y=0.000000)"))))
    (:then_1
      (Utilities|IsValid (LocalVariables|GetPrevious)
        (:Is%20Valid
          ;[1 1 1] Set the code piece at the appropriate location.
          (Variables|/Game/Deadbit/Blueprints/BotProgramming/Functions/BaseClasses/CodePiece.CodePiece_C|SetGridX (LocalVariables|GetPiece) (+ (Variables|/Game/Deadbit/Blueprints/BotProgramming/Functions/BaseClasses/CodePiece.CodePiece_C|GetGridX (LocalVariables|GetPrevious)) (Math|Float|Truncate (.x (LocalVariables|GetOffset)))))
          (Variables|/Game/Deadbit/Blueprints/BotProgramming/Functions/BaseClasses/CodePiece.CodePiece_C|SetGridY (LocalVariables|GetPiece) (+ (Variables|/Game/Deadbit/Blueprints/BotProgramming/Functions/BaseClasses/CodePiece.CodePiece_C|GetGridY (LocalVariables|GetPrevious)) (Math|Float|Truncate (.y (LocalVariables|GetOffset)))))
          (Utilities|Array|SetArrayElem (Variables|/Game/Deadbit/Blueprints/BotProgramming/Functions/BaseClasses/CodePiece.CodePiece_C|GetNextInstructions (LocalVariables|GetPrevious)) 0 (LocalVariables|GetPiece)))
        (:Is%20Not%20Valid
          (bind _output_get (Variables|Default|SetFirstCodePiece (LocalVariables|GetPiece)))
          (Variables|/Game/Deadbit/Blueprints/BotProgramming/Functions/BaseClasses/CodePiece.CodePiece_C|SetGridX _output_get 3)
          (Variables|/Game/Deadbit/Blueprints/BotProgramming/Functions/BaseClasses/CodePiece.CodePiece_C|SetGridY _output_get 2))))))

(fn Abort
  (bind _currentcodepiece (Variables|Default|GetCurrentCodePiece))
  (Utilities|IsValid _currentcodepiece
    (:Is%20Valid
      (Default|Abort (.AsVoid%20Piece (Utilities|Casting|CastToVoidPiece _currentcodepiece)))
      (Variables|Default|SetProgramRunning false))))

(fn ContainsInstruction
  (params (Instruction%20Type :type Code%20Piece%20Class%20Reference))
  (bind _values (Utilities|Map|Values (Variables|Default|GetProgramStructure)))
  (for _array_element _values
    (if (== (Utilities|GetClass (Variables|/Game/Deadbit/Blueprints/UI/ProgrammingUI/ChipWidgetOld.ChipWidgetOld_C|GetCodePiece _array_element)) Instruction%20Type)
      (return true)
      (else
        (for _array_element_2 (Variables|/Game/Deadbit/Blueprints/BotProgramming/Functions/BaseClasses/CodePiece.CodePiece_C|GetParameters (Variables|/Game/Deadbit/Blueprints/UI/ProgrammingUI/ChipWidgetOld.ChipWidgetOld_C|GetCodePiece _array_element))
          (if (== Instruction%20Type (Utilities|GetClass _array_element_2))
            (return true))))))
  (return false))

(fn GetAdjacent(Vector2D)
  (params (Key :type Int%20Point%20Structure))
  (return (Utilities|IntPoint+IntPoint Key (Utilities|Struct|MakeIntPoint 0 1)) (Utilities|IntPoint+IntPoint Key (Utilities|Struct|MakeIntPoint -1 0)) (Utilities|IntPoint+IntPoint Key (Utilities|Struct|MakeIntPoint 1 0)) (Utilities|IntPoint+IntPoint Key (Utilities|Struct|MakeIntPoint 0 -1))))

(fn GetAdjacent(CodePiece)
  (params (Code%20Piece :type Code%20Piece%20Object%20Reference) (Key :type Int%20Point%20Structure))
  (bind (_upadjacent _leftadjacent _rightadjacent _downadjacent) (CallFunction|GetAdjacent(Vector2D) Key))
  (for _array_element (Utilities|Array|MakeArray _upadjacent _leftadjacent _rightadjacent _downadjacent)
    (if (.ReturnValue (Utilities|Map|Find (Variables|Default|GetProgramStructure) _array_element))
      (Utilities|Array|Add (LocalVariables|GetAdjacent) (.Value (Utilities|Map|Find (Variables|Default|GetProgramStructure) _array_element)))))
  (return (LocalVariables|GetAdjacent)))

(fn GetNext
  (params (Direction :type Direction%20Enum :default "NewEnumerator0") (CurrentKey :type Int%20Point%20Structure))
  (switch Utilities|FlowControl|Switch|SwitchonDirection Direction
    (:NewEnumerator0
      (return (Utilities|IntPoint+IntPoint CurrentKey (Utilities|Struct|MakeIntPoint 0 -1))))
    (:NewEnumerator3
      (return (Utilities|IntPoint+IntPoint CurrentKey (Utilities|Struct|MakeIntPoint 1 0))))
    (:NewEnumerator1
      (return (Utilities|IntPoint+IntPoint CurrentKey (Utilities|Struct|MakeIntPoint 0 1))))
    (:NewEnumerator2
      (return (Utilities|IntPoint+IntPoint CurrentKey (Utilities|Struct|MakeIntPoint -1 0))))))

(fn AddCodePiecebyClass
  (params (Index :type Int%20Point%20Structure) (Code%20Piece%20Class :type Code%20Piece%20Class%20Reference))
  (return 0))