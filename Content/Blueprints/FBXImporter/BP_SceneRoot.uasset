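; BP_SceneRoot is the FBX importer's scene registry, tracking BP_SceneNode actors by name and driving named switches.
; On BeginPlay, if Node2Name is empty, it sets itself as each node's SceneRoot and registers it.
; Registration keeps two-way maps, with array structs allowing several nodes per name, and removes stale entries on re-registration.
; SetSwitch applies a value to every BP_Switch under a SwitchMap name, which is not populated here.
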(event EventBeginPlay
  (if (== (Utilities|Map|Length (Variables|Default|GetNode2Name)) 0)
    (CallFunction|InitializeMaps)))

(fn ConstructionScript)

(fn SetSwitch
  (params (Name :type String) (Value :type Integer))
  (bind _switchmap (Variables|Default|GetSwitchMap))
  (bind (_value _returnvalue) (Utilities|Map|Find _switchmap Name))
  (if _returnvalue
    (for _array_element (Utilities|Struct|BreakArrayOfSwitch _value)
      (bind _asbp_switch (Utilities|Casting|CastToBP_Switch _array_element))
      (Default|SetSelection _asbp_switch Value))
    (else
      (Development|PrintString (Utilities|String|Append "Error: switch \"" Name "\" was not found") true true "(R=0.552083,G=0.000000,B=0.000000,A=1.000000)" 3.0))))

(fn RegisterSceneNode
  (params (Node :type BP%20Scene%20Node%20Object%20Reference) (NameID :type Name))
  (bind _name2node (Variables|FBXImporter|GetName2Node))
  (bind _node2name (Variables|Default|GetNode2Name))
  (bind _name2node_2 (Variables|FBXImporter|GetName2Node))
  (bind (_value _returnvalue) (Utilities|Map|Find _node2name Node))
  (bind _value_2 (Utilities|Map|Find _name2node_2 NameID))
  (bind _value_3 (Utilities|Map|Find _name2node _value))
  (Utilities|FlowControl|Sequence
    (:then_0
      ;[1 1 1] First check if node already registered and remove it from register
      (if _returnvalue
        (bind _output_get (LocalVariables|SetTempNodeArray (Utilities|Struct|BreakArrayOfActor _value_3)))
        (Utilities|Array|RemoveItem _output_get Node)
        (bind _structout (Utilities|Struct|SetmembersinArrayOfActor _value_3 _output_get))
        (Utilities|Map|Add (Variables|FBXImporter|GetName2Node) _value _structout)))
    (:then_1
      (Utilities|Map|Add (Variables|Default|GetNode2Name) Node NameID)
      (bind _output_get_2 (LocalVariables|SetTempNodeArray (Utilities|Struct|BreakArrayOfActor _value_2)))
      (Utilities|Array|Add _output_get_2 Node)
      (bind _structout_2 (Utilities|Struct|SetmembersinArrayOfActor _value_2 _output_get_2))
      (Utilities|Map|Add (Variables|FBXImporter|GetName2Node) NameID _structout_2))))

(fn GetAllActiveActors
  (bind _outactors (Actor|GetAllActorsOfClass "/DatasmithContent/Blueprints/FBXImporter/BP_SceneNode.BP_SceneNode_C"))
  (return _outactors))

(fn InitializeMaps
  (bind _outactors (Actor|GetAllActorsOfClass "/DatasmithContent/Blueprints/FBXImporter/BP_SceneNode.BP_SceneNode_C"))
  (for _array_element _outactors
    (Variables|/DatasmithContent/Blueprints/FBXImporter/BP_SceneNode.BP_SceneNode_C|SetSceneRoot _array_element self)
    (CallFunction|RegisterSceneNode _array_element (Variables|/DatasmithContent/Blueprints/FBXImporter/BP_SceneNode.BP_SceneNode_C|GetNameID _array_element))))