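; BP_Switch is an FBX importer scene node that shows one of several attached child nodes at a time, like a variant selector.
; It maps attached BP_SceneNode actors to Options by NameID, rebuilding the mapping in SetSelection without a SceneRoot, so it works outside play.
; BeginPlay registers it by name in SceneRoot's SwitchMap, grouping same-named instances, and selects the first option.
; Selection cycles with wraparound, and node visibility changes affect only the selected child.
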(event EventBeginPlay
  (|CallParentFunction)
  (Utilities|FlowControl|Sequence
    (:then_0
      ;[1 1 1] Collect child actors used in Switch options
      (Utilities|Array|Resize (Variables|Default|GetOptionsActors) (Utilities|Array|Length (Variables|Default|GetOptions)))
      (for _array_element (Actor|GetAttachedActors)
        (bind _asbp_scene_node (Utilities|Casting|CastToBP_SceneNode _array_element))
        (if (!= (Utilities|Array|FindItem (Variables|Default|GetOptions) (Variables|/DatasmithContent/Blueprints/FBXImporter/BP_SceneNode.BP_SceneNode_C|GetNameID _asbp_scene_node)) -1)
          (Utilities|Array|SetArrayElem (Variables|Default|GetOptionsActors) (Utilities|Array|FindItem (Variables|Default|GetOptions) (Variables|/DatasmithContent/Blueprints/FBXImporter/BP_SceneNode.BP_SceneNode_C|GetNameID _asbp_scene_node)) _array_element))))
    (:then_1
      (CallFunction|RegisterSwitch)
      (CallFunction|SetSelection))))

(event EventOnSetNodeVisibility
  (params (NewVisibility :type Boolean))
  (bind _currentselection (Variables|Default|GetCurrentSelection))
  (bind _optionsactors (Variables|Default|GetOptionsActors))
  ;[0.08033 0.1094 0.03602] Only show or hide current selection child
  (if (Utilities|Array|IsValidIndex _optionsactors _currentselection)
    (CallFunction|SetActorVisibilityRecursive (Utilities|Array|Get(acopy) _optionsactors _currentselection) NewVisibility)
    (else
      ;[0.1664 0.157 0.3802] Uninitialized switch, should hide everything
      (if (== _currentselection -1)
        _))))

(fn ConstructionScript
  (|CallParentFunction))

(fn SetSelection
  (params (Value :type Integer))
  (Variables|Default|SetCurrentSelection Value)
  ;[0.5052 0.08618 0.1671] Only change when not hidden
  (if (Variables|Default|GetIsVisible)
    ;[1 1 1] If we have a SceneRoot, we're in play mode/runtime, so we already have a valid OptionsActors
    (Utilities|IsValid (Variables|Default|GetSceneRoot)
      (:Is%20Valid
        _)
      (:Is%20Not%20Valid
        ;[1 1 1] Build a temporary OptionsActors array with our current attachments
        (Utilities|Array|Resize (Variables|Default|GetOptionsActors) (Utilities|Array|Length (Variables|Default|GetOptions)))
        (for _array_element (Actor|GetAttachedActors)
          (bind _asbp_scene_node (Utilities|Casting|CastToBP_SceneNode _array_element))
          (if (!= (Utilities|Array|FindItem (Variables|Default|GetOptions) (Variables|/DatasmithContent/Blueprints/FBXImporter/BP_SceneNode.BP_SceneNode_C|GetNameID _asbp_scene_node)) -1)
            (Utilities|Array|SetArrayElem (Variables|Default|GetOptionsActors) (Utilities|Array|FindItem (Variables|Default|GetOptions) (Variables|/DatasmithContent/Blueprints/FBXImporter/BP_SceneNode.BP_SceneNode_C|GetNameID _asbp_scene_node)) _array_element)))))
    ;[0.0217 0.04413 0.1615] Process children
    (for (_array_element_2 _array_index) (Variables|Default|GetOptionsActors)
      (Utilities|IsValid _array_element_2
        (:Is%20Valid
          (CallFunction|SetActorVisibilityRecursive _array_element_2 (== _array_index (Variables|Default|GetCurrentSelection))))))))

(fn RegisterSwitch
  (bind _sceneroot (Variables|Default|GetSceneRoot))
  (bind _name (Variables|Default|GetName))
  (bind _switchmap (Variables|/DatasmithContent/Blueprints/FBXImporter/BP_SceneRoot.BP_SceneRoot_C|GetSwitchMap _sceneroot))
  (bind (_value _returnvalue) (Utilities|Map|Find _switchmap _name))
  ;[0.2656 0.1847 0.09287] We'll register this BP_Switch in root node, but only in root node exists
  (if (Utilities|IsValid (Variables|Default|GetSceneRoot))
    (if _returnvalue
      ;[0.09876 0.1536 0.2656] Add another instance of this switch
      (bind _output_get (LocalVariables|SetSwitchList (Utilities|Struct|BreakArrayOfSwitch _value)))
      (Utilities|Array|Add _output_get self)
      (Utilities|Map|Add _switchmap (Variables|Default|GetName) (Utilities|Struct|MakeArrayOfSwitch (LocalVariables|GetSwitchList)))
      (else
        ;[0.1587 0.224 0.03985] No switches with same name were registered, add first instance
        (Utilities|Map|Add _switchmap _name (Utilities|Struct|MakeArrayOfSwitch (Utilities|Array|MakeArray self)))))))

(fn SelectPrevious
  (bind _output_get (LocalVariables|SetNewSelection (- (Variables|Default|GetCurrentSelection) 1)))
  (if (< _output_get 0)
    (LocalVariables|SetNewSelection (- (Utilities|Array|Length (Variables|Default|GetOptions)) 1)))
  (CallFunction|SetSelection (LocalVariables|GetNewSelection)))

(fn SelectNext
  (bind _output_get (LocalVariables|SetNewSelection (+ (Variables|Default|GetCurrentSelection) 1)))
  (if (>= _output_get (Utilities|Array|Length (Variables|Default|GetOptions)))
    (LocalVariables|SetNewSelection 0))
  (CallFunction|SetSelection (LocalVariables|GetNewSelection)))