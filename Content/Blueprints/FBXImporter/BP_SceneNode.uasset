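; BP_SceneNode is a scene-node actor in the FBX importer that propagates visibility changes through its attached actor hierarchy.
; SetNodeVisibility acts on the first call or a changed value, then calls the overridable OnSetNodeVisibility.
; Attached actors update recursively: nested scene nodes handle themselves, while other actors set each scene component and descend into their attachments.
; A Debug macro gates debug code on the SceneRoot's flag or a force input.
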(event Collision|EventActorBeginOverlap
  (params (OtherActor :type Actor%20Object%20Reference)))

(event EventTick
  (params (DeltaSeconds :type Float%20%28single-precision%29)))

(fn ConstructionScript)

(fn SetNodeVisibility
  (params (NewVisible :type Boolean))
  ;[0.1142 0.1823 0.09018] Check if visibility for this node changed
  (if (Variables|Default|GetIsInitialized)
    (if (Math|Boolean|NotEqual(Boolean) (Variables|Default|GetIsVisible) NewVisible)
      (Variables|Default|SetIsVisible NewVisible :!label _label)
      ;[0.125 0.09783 0.04097] Change visibility (virtual function call)
      (CallFunction|OnSetNodeVisibility NewVisible))
    (else
      (Variables|Default|SetIsInitialized true)
      (goto _label))))

(fn SetActorVisibilityRecursive
  (params (Node :type Actor%20Object%20Reference) (NewVisible :type Boolean))
  (bind _asbp_scene_node (Utilities|Casting|CastToBP_SceneNode Node)
    (:then
      (CallFunction|SetNodeVisibility _asbp_scene_node NewVisible) ; BP_SceneNode processed separately
    )
    (:CastFailed
      (Utilities|FlowControl|Sequence
        (:then_0
          ;[0.2952 0.4062 0.1518] Process attached components
          (bind _output_get (LocalVariables|SetComponents (Actor|GetComponentsByClass Node "/Script/Engine.SceneComponent")))
          (for _array_element _output_get
            (Rendering|SetVisibility _array_element NewVisible false)))
        (:then_1
          ;[0.1166 0.1063 0.2865] Process attached actors
          (bind _output_get_2 (LocalVariables|SetChildActors (Actor|GetAttachedActors Node)))
          (for _array_element_2 _output_get_2
            (CallFunction|SetActorVisibilityRecursive _array_element_2 NewVisible)))))))

(fn OnSetNodeVisibility
  (params (NewVisibility :type Boolean))
  (bind _output_get (LocalVariables|SetActors (Actor|GetAttachedActors)))
  (for _array_element _output_get
    (CallFunction|SetActorVisibilityRecursive _array_element NewVisibility)))

(fn GetRoot
  (return (Variables|Default|GetSceneRoot)))