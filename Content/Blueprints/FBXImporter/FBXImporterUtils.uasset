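; Blueprint utility functions for the FBX importer that query imported actor hierarchies.
; GetAllAttachedActors gathers every attached descendant of a root actor through a recursive internal helper that appends to a shared result array.
; Name lookups read the root's Name2Node map, returning either all name IDs or the list stored under a given ID.
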(fn GetAllAttachedActorsInternal
  (params (RootActor :type Actor%20Object%20Reference) (Result :type Array%20of%20Actor%20Object%20References))
  (for _array_element (Actor|GetAttachedActors RootActor)
    (Utilities|FlowControl|Sequence
      (:then_0
        (Utilities|Array|Add Result _array_element))
      (:then_1
        (CallFunction|GetAllAttachedActorsInternal _array_element Result)))))

(fn GetAllAttachedActors
  (params (RootActor :type Actor%20Object%20Reference))
  (bind _result (LocalVariables|GetResult))
  (CallFunction|GetAllAttachedActorsInternal RootActor _result)
  (return _result))

(fn GetActorsforNameID
  (params (NameID :type Name%20%28by%20ref%29) (Root :type BP%20Scene%20Root%20Object%20Reference))
  (return (Utilities|Struct|BreakArrayOfActor (.Value (Utilities|Map|Find (Variables|/DatasmithContent/Blueprints/FBXImporter/BP_SceneRoot.BP_SceneRoot_C|GetName2Node Root) NameID)))))

(fn GetActorsNameIDs
  (params (Root :type BP%20Scene%20Root%20Object%20Reference))
  (bind _keys (Utilities|Map|Keys (Variables|/DatasmithContent/Blueprints/FBXImporter/BP_SceneRoot.BP_SceneRoot_C|GetName2Node Root)))
  (return _keys))